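; Placeable suburban fence piece that sets its mesh and material in the Construction Script from editable options, with no active gameplay logic.
; The selected model (short, tall, angled or post) indexes one of several mesh arrays, chosen by modular, left/right direction and damaged settings.
; A custom material list supplies the first material slot.
; Userfriendly clamps out-of-range material indices with a warning and nudges the model and direction arrays toward single entries.
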(fn `ChooseMesh`
  (params (SelectionIndex :type Integer))
  (if (`self.Modular`)
    (switch `/Game/Suburban_Modular_Fence/Blueprints/Enums/E_Direction` (`|GetArrayItem` (`self.Direction`))
      (:`NewEnumerator0`
        (if (`self.IsDamaged?`)
          (`StaticMeshComponent.SetStaticMesh` (`self.Mesh`) (`|GetArrayItem` (`self.Damaged_Fence_Types_Left`) SelectionIndex))
          (else
            (`StaticMeshComponent.SetStaticMesh` (`self.Mesh`) (`|GetArrayItem` (`self.Fence_Types_Left`) SelectionIndex)))))
      (:`NewEnumerator1`
        (if (`self.IsDamaged?`)
          (`StaticMeshComponent.SetStaticMesh` (`self.Mesh`) (`|GetArrayItem` (`self.Damaged_Fence_Types_Right`) SelectionIndex))
          (else
            (`StaticMeshComponent.SetStaticMesh` (`self.Mesh`) (`|GetArrayItem` (`self.Fence_Types_Right`) SelectionIndex))))))
    (elif (`self.IsDamaged?`)
      (`StaticMeshComponent.SetStaticMesh` (`self.Mesh`) (`|GetArrayItem` (`self.Fence_Damaged_Nonmodular`) SelectionIndex))
      (else
        (`StaticMeshComponent.SetStaticMesh` (`self.Mesh`) (`|GetArrayItem` (`self.Fence_Nonmodular`) SelectionIndex)))))
  (return))

(fn `UserConstructionScript`
  (`|ExecutionSequence`
    (:`then_0`
      (`self.Userfriendly`)
      (switch `/Game/Suburban_Modular_Fence/Blueprints/Enums/E_ModelChoice` (`|GetArrayItem` (`self.Select Model:`))
        (:`NewEnumerator0`
          (`self.ChooseMesh` 0))
        (:`NewEnumerator1`
          (`self.ChooseMesh` 1))
        (:`NewEnumerator2`
          (`self.ChooseMesh` 2))
        (:`NewEnumerator3`
          (`self.ChooseMesh` 3))
        (:`NewEnumerator4`
          (`self.ChooseMesh` 4))
        (:`NewEnumerator5`
          (`self.ChooseMesh` 5))
        (:`NewEnumerator6`
          (`self.ChooseMesh` 6))
        (:`NewEnumerator7`
          (`self.ChooseMesh` 7))))
    (:`then_1`
      (`PrimitiveComponent.SetMaterial` (`self.Mesh`) 0 (`|GetArrayItem` (`self.Custom Material List (Assing your materials here)`) (`self.Select Material Index:`))))))

(fn `Userfriendly`
  (bind _select_model_ (`self.Select Model:`))
  (bind _direction (`self.Direction`))
  (bind _returnvalue (`KismetArrayLibrary.Array_Length` (`self.Custom Material List (Assing your materials here)`)))
  (bind _returnvalue_2 (`KismetArrayLibrary.Array_Length` _direction))
  (bind _returnvalue_3 (`KismetArrayLibrary.Array_Length` _select_model_))
  (if (> (+ (`self.Select Material Index:`) 1) _returnvalue)
    (`KismetSystemLibrary.PrintString` "Your material selection is out of bounds." true true (struct :`R` 0.71875 :`A` 1.0) 5.0)
    (set `self.Select Material Index:` (- _returnvalue 1))
    (elif (< (`self.Select Material Index:`) 0)
      (`KismetSystemLibrary.PrintString` "Your material selection is out of bounds." true true (struct :`R` 0.71875 :`A` 1.0) 5.0)
      (set `self.Select Material Index:` 0)
      (elif (> _returnvalue_3 1)
        (`KismetArrayLibrary.Array_Remove` _select_model_ 1)
        (elif (== _returnvalue_3 0)
          (`KismetArrayLibrary.Array_Add` _select_model_ "NewEnumerator0")
          (elif (> _returnvalue_2 1)
            (`KismetArrayLibrary.Array_Remove` _direction 1)
            (elif (== _returnvalue_2 0)
              (`KismetArrayLibrary.Array_Add` _direction "NewEnumerator0"))))))))