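; BP_WallShop is a placeable shop wall that sinks to open and rises to close.
; Open and Close play one timeline forward or in reverse, lerping the actor between two fixed world heights while keeping the X and Y cached at BeginPlay.
; Both events also set StartWave on a referenced button, false on Open and true on Close, tying the wall to wave state.
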(event `self.ReceiveBeginPlay`
  (set `self.DefLoc` (`self.K2_GetActorLocation`)))

(event `Open`
  (bind (_defloc_x _defloc_y) (`KismetMathLibrary.BreakVector` (`self.DefLoc`)))
  (set `/Game/Core/Items/BP_Button_Wave.Start Wave` false (`self.Ref Button`))
  (bind (_direction _alpha) (`Timeline|Opening` :!via `PlayFromStart` :!label _label)
    (:`Update`
      (`self.K2_SetActorLocation` (`KismetMathLibrary.MakeVector` _defloc_x _defloc_y (`KismetMathLibrary.Lerp` 110.0 -300.0 _alpha))))))

(event `Close`
  (set `/Game/Core/Items/BP_Button_Wave.Start Wave` true (`self.Ref Button`))
  (goto _label :!via `ReverseFromEnd`))

(fn `UserConstructionScript`)