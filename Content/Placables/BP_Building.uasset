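; BP_Building is a placeable actor that creates an endlessly descending building from two alternating pieces.
; On BeginPlay, a timeline running at PlayRate lowers the whole actor by Size per cycle.
; After each cycle it stores the new position, uses a FlipFlop to move Building1 or Building2 to an ever-higher relative Z offset, then restarts.
; This leapfrogging recycles the two components as a continuous vertical column.
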(event `self.ReceiveBeginPlay`
  (bind (_defloc_x _defloc_y _defloc_z) (`KismetMathLibrary.BreakVector` (`self.DefLoc`)))
  (bind _location (`self.Location`))
  (`TimelineComponent.SetPlayRate` (`self.Anim`) (`self.PlayRate`))
  (set `self.DefLoc` (`self.K2_GetActorLocation`))
  (bind (_direction _alpha) (`Timeline|Anim` :!via `PlayFromStart` :!label _label)
    (:`Update`
      (`self.K2_SetActorLocation` (`KismetMathLibrary.MakeVector` _defloc_x _defloc_y (`KismetMathLibrary.Lerp` _defloc_z (- _defloc_z (`self.Size`)) _alpha))))
    (:`Finished`
      (set `self.DefLoc` (`self.K2_GetActorLocation`))
      (`/Engine/EditorBlueprintResources/StandardMacros.FlipFlop`
        (:`A`
          (`SceneComponent.K2_SetRelativeLocation` (`self.Building1`) (`KismetMathLibrary.MakeVector` 0.0 0.0 _location) false false))
        (:`B`
          (`SceneComponent.K2_SetRelativeLocation` (`self.Building2`) (`KismetMathLibrary.MakeVector` 0.0 0.0 _location) false false)))
      (set `self.Location` (+ (`self.Location`) 3600.0))
      (`self.Loop`))))

(event `Loop`
  (goto _label :!via `PlayFromStart`))

(fn `UserConstructionScript`)