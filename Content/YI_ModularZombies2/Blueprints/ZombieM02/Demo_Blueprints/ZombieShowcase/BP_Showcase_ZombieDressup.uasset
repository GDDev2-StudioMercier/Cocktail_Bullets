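; Showcase actor that dresses up a modular male zombie (M02) with selectable body type, clothing, hair, gore and material variants for demo display.
; The construction script makes the clothing meshes follow the body's pose as leader, then applies the selection variables to visibility, meshes and materials, with head materials depending on body type.
; It also configures two optional showcase lights; Tick yaws a Box component in delayed steps while light rotation is enabled.
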(event `self.ReceiveTick`
  (params (DeltaSeconds :type "Float (single-precision)"))
  (bind _box (`self.Box`))
  (bind (_returnvalue_roll _returnvalue_pitch _returnvalue_yaw) (`KismetMathLibrary.BreakRotator` (`SceneComponent.K2_GetComponentRotation` _box)))
  (if (`self.ShowcaseLightsRotate?`)
    (`KismetSystemLibrary.Delay` (`self.RotationTickDelay`))
    (`SceneComponent.K2_SetWorldRotation` _box (`KismetMathLibrary.MakeRotator` _returnvalue_roll _returnvalue_pitch (+ _returnvalue_yaw (`self.RotationPerTick`))) false false)))

(fn `UserConstructionScript`
  (bind _sk_zombiemale02 (`self.SK_ZombieMale02`))
  (bind _sk_clothing_longpants (`self.SK_Clothing_LongPants`))
  (bind _sk_clothing_tshirt (`self.SK_Clothing_Tshirt`))
  (bind _sk_clothing_singlet (`self.SK_Clothing_Singlet`))
  (bind _sk_zombiemale02_2 (`self.SK_ZombieMale02`))
  (bind _sk_clothing_singlet_2 (`self.SK_Clothing_Singlet`))
  (bind _hair_01 (`self.Hair_01`))
  (bind _sk_zombiemale02_3 (`self.SK_ZombieMale02`))
  (bind _sk_clothing_longpants_2 (`self.SK_Clothing_LongPants`))
  (bind _selectzombie (`self.SelectZombie`))
  (bind _sk_clothing_tshirt_2 (`self.SK_Clothing_Tshirt`))
  (`SkinnedMeshComponent.SetLeaderPoseComponent` (`self.SK_Clothing_Tshirt`) (`self.SK_ZombieMale02`) false false)
  (`SkinnedMeshComponent.SetLeaderPoseComponent` (`self.SK_Clothing_LongPants`) (`self.SK_ZombieMale02`) false false)
  (`SkinnedMeshComponent.SetLeaderPoseComponent` (`self.SK_Clothing_Singlet`) (`self.SK_ZombieMale02`) false false)
  (`|ExecutionSequence`
    (:`then_0`
      ;[1 1 1] Select Mesh Options
      (`|ExecutionSequence`
        (:`then_0`
          (switch `/Game/YI_ModularZombies2/Blueprints/ZombieM02/Demo_Blueprints/ZombieShowcase/Enums/E_PantsType` (`self.SelectPants`)
            (:`NewEnumerator0`
              (`SceneComponent.SetVisibility` _sk_clothing_longpants_2 false false))
            (:`NewEnumerator1`
              (`SceneComponent.SetVisibility` _sk_clothing_longpants_2 true false))))
        (:`then_1`
          (switch `/Game/YI_ModularZombies2/Blueprints/ZombieM02/Demo_Blueprints/ZombieShowcase/Enums/E_ShirtType` (`self.SelectShirt`)
            (:`NewEnumerator0`
              (`SceneComponent.SetVisibility` _sk_clothing_tshirt false false)
              (`SceneComponent.SetVisibility` _sk_clothing_singlet false false))
            (:`NewEnumerator2`
              (`SceneComponent.SetVisibility` _sk_clothing_singlet true false)
              (`SceneComponent.SetVisibility` _sk_clothing_tshirt false false))
            (:`NewEnumerator3`
              (`SceneComponent.SetVisibility` _sk_clothing_tshirt true false)
              (`SceneComponent.SetVisibility` _sk_clothing_singlet false false))))
        (:`then_2`
          (switch `/Game/YI_ModularZombies2/Blueprints/ZombieM02/Demo_Blueprints/ZombieShowcase/Enums/E_ZombieType` (`self.SelectZombie`)
            (:`NewEnumerator0`
              (`SkinnedMeshComponent.SetSkinnedAssetAndUpdate` _sk_zombiemale02 "/Game/YI_ModularZombies2/Meshes/ZombieM02/Zombie/SK_Zombie_M02_01.SK_Zombie_M02_01" true))
            (:`NewEnumerator1`
              (`SkinnedMeshComponent.SetSkinnedAssetAndUpdate` _sk_zombiemale02 "/Game/YI_ModularZombies2/Meshes/ZombieM02/Zombie/SK_Zombie_M02_02.SK_Zombie_M02_02" true))))
        (:`then_3`
          (switch `/Game/YI_ModularZombies2/Blueprints/ZombieM02/Demo_Blueprints/ZombieShowcase/Enums/E_HeadAccessoryType` (`self.SelectHeadAccessory`)
            (:`NewEnumerator0`
              (`SceneComponent.SetVisibility` _hair_01 false false))
            (:`NewEnumerator2`
              (`SceneComponent.SetVisibility` _hair_01 true false)
              (`StaticMeshComponent.SetStaticMesh` (`self.Hair_01`) "/Game/YI_ModularZombies2/Meshes/ZombieM02/Hair/SM_HairCombined_M02.SM_HairCombined_M02"))))))
    (:`then_1`
      (`|ExecutionSequence`
        (:`then_0`
          ;[1 1 1] Body
          (switch `/Game/YI_ModularZombies2/Blueprints/ZombieM02/Demo_Blueprints/ZombieShowcase/Enums/E_ZombieMaterialVariations` (`self.Select Zombie Base Material`)
            (:`NewEnumerator0`
              (`PrimitiveComponent.SetMaterialByName` _sk_zombiemale02_2 "Body" "/Game/YI_ModularZombies2/Materials/ZombieM02/Body/Var1NoGore/MI_Body_Zombie_M02_01.MI_Body_Zombie_M02_01"))
            (:`NewEnumerator6`
              (`PrimitiveComponent.SetMaterialByName` _sk_zombiemale02_2 "Body" "/Game/YI_ModularZombies2/Materials/ZombieM02/Body/Var2ChestGore/MI_Body_Zombie_M02_02.MI_Body_Zombie_M02_02"))
            (:`NewEnumerator7`
              (`PrimitiveComponent.SetMaterialByName` _sk_zombiemale02_2 "Body" "/Game/YI_ModularZombies2/Materials/ZombieM02/Body/Var3BodyBitten/MI_Body_Zombie_M02_03.MI_Body_Zombie_M02_03"))
            (:`NewEnumerator8`
              (`PrimitiveComponent.SetMaterialByName` _sk_zombiemale02_2 "Body" "/Game/YI_ModularZombies2/Materials/ZombieM02/Body/Var4BittenChestGore/MI_Body_Zombie_M02_04.MI_Body_Zombie_M02_04"))))
        (:`then_1`
          ;[1 1 1] HeadVariations
          (switch `/Game/YI_ModularZombies2/Blueprints/ZombieM02/Demo_Blueprints/ZombieShowcase/Enums/E_ZombieHeadVariations` (`self.Select Zombie Head Base Material`)
            (:`NewEnumerator0`
              (switch `/Game/YI_ModularZombies2/Blueprints/ZombieM02/Demo_Blueprints/ZombieShowcase/Enums/E_ZombieType` _selectzombie
                (:`NewEnumerator0`
                  (`PrimitiveComponent.SetMaterialByName` _sk_zombiemale02_3 "Head" "/Game/YI_ModularZombies2/Materials/ZombieM02/Head01/Var1NoGore/MI_Head01_Zombie_M02_01.MI_Head01_Zombie_M02_01"))
                (:`NewEnumerator1`
                  (`PrimitiveComponent.SetMaterialByName` _sk_zombiemale02_3 "Head" "/Game/YI_ModularZombies2/Materials/ZombieM02/Head02/Var1NoGore/MI_Head02_Zombie_M02_01.MI_Head02_Zombie_M02_01"))))
            (:`NewEnumerator6`
              (switch `/Game/YI_ModularZombies2/Blueprints/ZombieM02/Demo_Blueprints/ZombieShowcase/Enums/E_ZombieType` _selectzombie
                (:`NewEnumerator0`
                  (`PrimitiveComponent.SetMaterialByName` _sk_zombiemale02_3 "Head" "/Game/YI_ModularZombies2/Materials/ZombieM02/Head01/Var2CheekWound/MI_Head01_Zombie_M02_02.MI_Head01_Zombie_M02_02"))
                (:`NewEnumerator1`
                  (`PrimitiveComponent.SetMaterialByName` _sk_zombiemale02_3 "Head" "/Game/YI_ModularZombies2/Materials/ZombieM02/Head02/Var2HeadWoundOnly/MI_Head02_Zombie_M02_02.MI_Head02_Zombie_M02_02"))))
            (:`NewEnumerator7`
              (switch `/Game/YI_ModularZombies2/Blueprints/ZombieM02/Demo_Blueprints/ZombieShowcase/Enums/E_ZombieType` _selectzombie
                (:`NewEnumerator0`
                  (`PrimitiveComponent.SetMaterialByName` _sk_zombiemale02_3 "Head" "/Game/YI_ModularZombies2/Materials/ZombieM02/Head01/Var3FullWounds/MI_Head01_Zombie_M02_03.MI_Head01_Zombie_M02_03"))
                (:`NewEnumerator1`
                  (`PrimitiveComponent.SetMaterialByName` _sk_zombiemale02_3 "Head" "/Game/YI_ModularZombies2/Materials/ZombieM02/Head02/Var3GoreMouth/MI_Head02_Zombie_M02_03.MI_Head02_Zombie_M02_03"))))
            (:`NewEnumerator8`
              (switch `/Game/YI_ModularZombies2/Blueprints/ZombieM02/Demo_Blueprints/ZombieShowcase/Enums/E_ZombieType` _selectzombie
                (:`NewEnumerator0`
                  (`PrimitiveComponent.SetMaterialByName` _sk_zombiemale02_3 "Head" "/Game/YI_ModularZombies2/Materials/ZombieM02/Head01/Var4MouthGoreOnly/MI_Head01_Zombie_M02_04.MI_Head01_Zombie_M02_04"))
                (:`NewEnumerator1`
                  (`PrimitiveComponent.SetMaterialByName` _sk_zombiemale02_3 "Head" "/Game/YI_ModularZombies2/Materials/ZombieM02/Head02/Var4MouthOnly/MI_Head02_Zombie_M02_04.MI_Head02_Zombie_M02_04"))))))
        (:`then_2`
          ;[1 1 1] LongPants
          (switch `/Game/YI_ModularZombies2/Blueprints/ZombieM02/Demo_Blueprints/ZombieShowcase/Enums/E_Clothing_LongPantsMaterialVariations` (`self.Select Long Pants Material`)
            (:`NewEnumerator0`
              (`PrimitiveComponent.SetMaterial` _sk_clothing_longpants 0 "/Game/YI_ModularZombies2/Materials/ZombieM02/Clothing/LongJeans/01BlueClean/MI_Clth_LongJeans_M02_01.MI_Clth_LongJeans_M02_01"))
            (:`NewEnumerator7`
              (`PrimitiveComponent.SetMaterial` _sk_clothing_longpants 0 "/Game/YI_ModularZombies2/Materials/ZombieM02/Clothing/LongJeans/02BlueDirty/MI_Clth_LongJeans_M02_02.MI_Clth_LongJeans_M02_02"))
            (:`NewEnumerator8`
              (`PrimitiveComponent.SetMaterial` _sk_clothing_longpants 0 "/Game/YI_ModularZombies2/Materials/ZombieM02/Clothing/LongJeans/03KhakiClean/MI_Clth_LongJeans_M02_03.MI_Clth_LongJeans_M02_03"))
            (:`NewEnumerator9`
              (`PrimitiveComponent.SetMaterial` _sk_clothing_longpants 0 "/Game/YI_ModularZombies2/Materials/ZombieM02/Clothing/LongJeans/04KhakiDirty/MI_Clth_LongJeans_M02_04.MI_Clth_LongJeans_M02_04"))))
        (:`then_3`
          ;[1 1 1] Singlet
          (switch `/Game/YI_ModularZombies2/Blueprints/ZombieM02/Demo_Blueprints/ZombieShowcase/Enums/E_Clothing_SingletMaterialVariations` (`self.Select Singlet Material`)
            (:`NewEnumerator0`
              (`PrimitiveComponent.SetMaterial` _sk_clothing_singlet_2 0 "/Game/YI_ModularZombies2/Materials/ZombieM02/Clothing/Singlet/01WhiteClean/MI_Clth_Singlet_M02_01.MI_Clth_Singlet_M02_01"))
            (:`NewEnumerator6`
              (`PrimitiveComponent.SetMaterial` _sk_clothing_singlet_2 0 "/Game/YI_ModularZombies2/Materials/ZombieM02/Clothing/Singlet/02WhiteDirty/MI_Clth_Singlet_M02_02.MI_Clth_Singlet_M02_02"))
            (:`NewEnumerator7`
              (`PrimitiveComponent.SetMaterial` _sk_clothing_singlet_2 0 "/Game/YI_ModularZombies2/Materials/ZombieM02/Clothing/Singlet/03WhiteGore/MI_Clth_Singlet_M02_03.MI_Clth_Singlet_M02_03"))
            (:`NewEnumerator8`
              (`PrimitiveComponent.SetMaterial` _sk_clothing_singlet_2 0 "/Game/YI_ModularZombies2/Materials/ZombieM02/Clothing/Singlet/04BlueGore/MI_Clth_Singlet_M02_04.MI_Clth_Singlet_M02_04"))
            (:`NewEnumerator9`
              (`PrimitiveComponent.SetMaterial` _sk_clothing_singlet_2 0 "/Game/YI_ModularZombies2/Materials/ZombieM02/Clothing/Singlet/05SafetyVest/MI_Clth_Singlet_M02_05.MI_Clth_Singlet_M02_05"))
            (:`NewEnumerator10`
              (`PrimitiveComponent.SetMaterial` _sk_clothing_singlet_2 0 "/Game/YI_ModularZombies2/Materials/ZombieM02/Clothing/Singlet/06RedWhiteStyled/MI_Clth_Singlet_M02_06.MI_Clth_Singlet_M02_06"))))
        (:`then_4`
          ;[1 1 1] Tshirt
          (switch `/Game/YI_ModularZombies2/Blueprints/ZombieM02/Demo_Blueprints/ZombieShowcase/Enums/E_Clothing_TShirtMaterialVariations` (`self.Select Tshirt Material`)
            (:`NewEnumerator0`
              (`PrimitiveComponent.SetMaterial` _sk_clothing_tshirt_2 0 "/Game/YI_ModularZombies2/Materials/ZombieM02/Clothing/Tshirt/01WhiteClean/MI_Clth_Tshirts_M02_01.MI_Clth_Tshirts_M02_01"))
            (:`NewEnumerator6`
              (`PrimitiveComponent.SetMaterial` _sk_clothing_tshirt_2 0 "/Game/YI_ModularZombies2/Materials/ZombieM02/Clothing/Tshirt/02WhiteDirty/MI_Clth_Tshirts_M02_02.MI_Clth_Tshirts_M02_02"))
            (:`NewEnumerator7`
              (`PrimitiveComponent.SetMaterial` _sk_clothing_tshirt_2 0 "/Game/YI_ModularZombies2/Materials/ZombieM02/Clothing/Tshirt/03BlackGore/MI_Clth_Tshirts_M02_03.MI_Clth_Tshirts_M02_03"))
            (:`NewEnumerator8`
              (`PrimitiveComponent.SetMaterial` _sk_clothing_tshirt_2 0 "/Game/YI_ModularZombies2/Materials/ZombieM02/Clothing/Tshirt/04WhiteGore/MI_Clth_Tshirts_M02_04.MI_Clth_Tshirts_M02_04"))
            (:`NewEnumerator9`
              (`PrimitiveComponent.SetMaterial` _sk_clothing_tshirt_2 0 "/Game/YI_ModularZombies2/Materials/ZombieM02/Clothing/Tshirt/05RedGore/MI_Clth_Tshirts_M02_05.MI_Clth_Tshirts_M02_05"))
            (:`NewEnumerator10`
              (`PrimitiveComponent.SetMaterial` _sk_clothing_tshirt_2 0 "/Game/YI_ModularZombies2/Materials/ZombieM02/Clothing/Tshirt/06GreenWhiteStripedGore/MI_Clth_Tshirts_M02_06.MI_Clth_Tshirts_M02_06"))))
        (:`then_5`
          ;[1 1 1] Hair Color
          (switch `/Game/YI_ModularZombies2/Blueprints/ZombieM02/Demo_Blueprints/ZombieShowcase/Enums/E_HairColorsMaterialVariations` (`self.Select Hair Color`)
            (:`NewEnumerator0`
              (`PrimitiveComponent.SetMaterial` (`self.Hair_01`) 1 "/Game/YI_ModularZombies2/Materials/ZombieM02/Hair/MI_Hair_Brown_M02.MI_Hair_Brown_M02"))))))
    (:`then_2`
      ;[1 1 1] Showcase Light Settings
      (if (`self.ShowcaseLightsOn?`)
        (`SceneComponent.SetVisibility` (`self.RotatingLight_01`) true false)
        (`SceneComponent.SetVisibility` (`self.RotatingLight_02`) true false)
        (if (`self.ShowcaseLightsShadows?`)
          (`LightComponentBase.SetCastShadows` (`self.RotatingLight_01`) true)
          (`LightComponentBase.SetCastShadows` (`self.RotatingLight_02`) true)
          (else
            (`LightComponentBase.SetCastShadows` (`self.RotatingLight_02`) false)
            (`LightComponentBase.SetCastShadows` (`self.RotatingLight_01`) false)))
        (else
          (`SceneComponent.SetVisibility` (`self.RotatingLight_02`) false false)
          (`SceneComponent.SetVisibility` (`self.RotatingLight_01`) false false)
          (set `self.ShowcaseLightsRotate?` false))))))