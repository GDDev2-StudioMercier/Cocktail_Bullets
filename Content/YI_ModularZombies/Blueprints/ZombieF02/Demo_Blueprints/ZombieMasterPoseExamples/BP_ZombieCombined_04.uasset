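; Demo Blueprint of a modular female zombie assembled from separate skeletal mesh parts using leader pose.
; The construction script makes the torso drive the head, both arms, singlet and skirt, leaving the hair mesh outside that link.
; On BeginPlay, SetBonePhysics scans bone names for "hair" and enables physics simulation on hair bodies below each match.
; An optional breast physics call on the torso is present but left disconnected.
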(event `self.ReceiveBeginPlay`
  (`self.SetBonePhysics`))

(fn `SetBonePhysics`
  (for _array_element (`self.BoneNames`)
    (if (`KismetStringLibrary.Contains` (`KismetStringLibrary.Conv_NameToString` _array_element) "hair")
      (`SkeletalMeshComponent.SetAllBodiesBelowSimulatePhysics` (`self.SK_Hair`) _array_element true false))))

(fn `UserConstructionScript`
  (`SkinnedMeshComponent.SetLeaderPoseComponent` (`self.SK_ZombieLimb_RightArm`) (`self.SK_Torso`) false false)
  (`SkinnedMeshComponent.SetLeaderPoseComponent` (`self.SK_ZombieLimb_LeftArm`) (`self.SK_Torso`) false false)
  (`SkinnedMeshComponent.SetLeaderPoseComponent` (`self.SK_Head`) (`self.SK_Torso`) false false)
  (`SkinnedMeshComponent.SetLeaderPoseComponent` (`self.SK_Singlet`) (`self.SK_Torso`) false false)
  (`SkinnedMeshComponent.SetLeaderPoseComponent` (`self.SK_Skirt`) (`self.SK_Torso`) false false))