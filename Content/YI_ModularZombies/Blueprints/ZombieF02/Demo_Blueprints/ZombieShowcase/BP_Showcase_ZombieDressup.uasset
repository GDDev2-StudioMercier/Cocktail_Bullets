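; Demo showcase actor for dressing up the modular Female 02 zombie with selectable body, head, clothing, hair and material variants.
; The construction script binds the garment and hair meshes to the body via leader pose, then applies the selection variables as mesh swaps, visibility toggles and material overrides, with head materials matched to zombie type.
; It also configures two optional showcase lights and their shadows, while Tick yaws the Box component when rotation is enabled.
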(event `self.ReceiveTick`
  (params (DeltaSeconds :type "Float (single-precision)"))
  (bind _box (`self.Box`))
  (bind (_returnvalue_roll _returnvalue_pitch _returnvalue_yaw) (`KismetMathLibrary.BreakRotator` (`SceneComponent.K2_GetComponentRotation` _box)))
  (if (`self.ShowcaseLightsRotate?`)
    (`KismetSystemLibrary.Delay` (`self.RotationTickDelay`))
    (`SceneComponent.K2_SetWorldRotation` _box (`KismetMathLibrary.MakeRotator` _returnvalue_roll _returnvalue_pitch (+ _returnvalue_yaw (`self.RotationPerTick`))) false false)))

(fn `UserConstructionScript`
  (bind _sk_zombiefemale02 (`self.SK_ZombieFemale02`))
  (bind _sk_cheerleader_skirt (`self.SK_Cheerleader_Skirt`))
  (bind _sk_money (`self.SK_Money`))
  (bind _sk_cheerleader_top (`self.SK_Cheerleader_Top`))
  (bind _sk_bralingerie (`self.SK_BraLingerie`))
  (bind _sk_hair (`self.SK_Hair`))
  (bind _sk_zombiefemale02_2 (`self.SK_ZombieFemale02`))
  (bind _sk_haircap (`self.SK_HairCap`))
  (bind _sk_cheerleader_skirt_2 (`self.SK_Cheerleader_Skirt`))
  (bind _sk_cheerleader_top_2 (`self.SK_Cheerleader_Top`))
  (bind _sk_bralingerie_2 (`self.SK_BraLingerie`))
  (bind _sk_hair_2 (`self.SK_Hair`))
  (bind _sk_zombiefemale02_3 (`self.SK_ZombieFemale02`))
  (bind _selectzombie (`self.SelectZombie`))
  (`SkinnedMeshComponent.SetLeaderPoseComponent` (`self.SK_Cheerleader_Skirt`) (`self.SK_ZombieFemale02`) false false)
  (`SkinnedMeshComponent.SetLeaderPoseComponent` (`self.SK_Cheerleader_Top`) (`self.SK_ZombieFemale02`) false false)
  (`SkinnedMeshComponent.SetLeaderPoseComponent` (`self.SK_BraLingerie`) (`self.SK_ZombieFemale02`) false false)
  (`SkinnedMeshComponent.SetLeaderPoseComponent` (`self.SK_HairCap`) (`self.SK_ZombieFemale02`) false false)
  (`SkinnedMeshComponent.SetLeaderPoseComponent` (`self.SK_Hair`) (`self.SK_ZombieFemale02`) false false)
  (`SkinnedMeshComponent.SetLeaderPoseComponent` (`self.SK_Money`) (`self.SK_ZombieFemale02`) false false)
  (`|ExecutionSequence`
    (:`then_0`
      ;[1 1 1] Select Mesh Options
      (`|ExecutionSequence`
        (:`then_0`
          (switch `/Game/YI_ModularZombies/Blueprints/ZombieF02/Demo_Blueprints/ZombieShowcase/Enums/E_PantsType` (`self.SelectPants`)
            (:`NewEnumerator0`
              (`SceneComponent.SetVisibility` _sk_money false false)
              (`SceneComponent.SetVisibility` _sk_cheerleader_skirt false false))
            (:`NewEnumerator1`
              (`SceneComponent.SetVisibility` _sk_cheerleader_skirt true false)
              (`SceneComponent.SetVisibility` _sk_money false false))
            (:`NewEnumerator3`
              (`SceneComponent.SetVisibility` _sk_money true false)
              (`SceneComponent.SetVisibility` _sk_cheerleader_skirt false false))))
        (:`then_1`
          (switch `/Game/YI_ModularZombies/Blueprints/ZombieF02/Demo_Blueprints/ZombieShowcase/Enums/E_ShirtType` (`self.SelectShirt`)
            (:`NewEnumerator0`
              (`SceneComponent.SetVisibility` _sk_cheerleader_top false false)
              (`SceneComponent.SetVisibility` _sk_bralingerie false false))
            (:`NewEnumerator2`
              (`SceneComponent.SetVisibility` _sk_bralingerie true false)
              (`SceneComponent.SetVisibility` _sk_cheerleader_top false false))
            (:`NewEnumerator3`
              (`SceneComponent.SetVisibility` _sk_cheerleader_top true false)
              (`SceneComponent.SetVisibility` _sk_bralingerie false false))))
        (:`then_2`
          (switch `/Game/YI_ModularZombies/Blueprints/ZombieF02/Demo_Blueprints/ZombieShowcase/Enums/E_ZombieType` (`self.SelectZombie`)
            (:`NewEnumerator0`
              (`SkinnedMeshComponent.SetSkinnedAssetAndUpdate` _sk_zombiefemale02 "/Game/YI_ModularZombies/Meshes/ZombieF02/Zombie/SK_Zombie_F02_01.SK_Zombie_F02_01" true))
            (:`NewEnumerator1`
              (`SkinnedMeshComponent.SetSkinnedAssetAndUpdate` _sk_zombiefemale02 "/Game/YI_ModularZombies/Meshes/ZombieF02/Zombie/SK_Zombie_F02_02.SK_Zombie_F02_02" true))))
        (:`then_3`
          (switch `/Game/YI_ModularZombies/Blueprints/ZombieF02/Demo_Blueprints/ZombieShowcase/Enums/E_HeadAccessoryType` (`self.SelectHeadAccessory`)
            (:`NewEnumerator0`
              (`SceneComponent.SetVisibility` _sk_hair false false)
              (`SceneComponent.SetVisibility` _sk_haircap false false))
            (:`NewEnumerator2`
              (`SceneComponent.SetVisibility` _sk_hair true false)
              (`SceneComponent.SetVisibility` _sk_haircap false false))
            (:`NewEnumerator3`
              (`SceneComponent.SetVisibility` _sk_haircap true false)
              (`SceneComponent.SetVisibility` _sk_hair false false))))))
    (:`then_1`
      (`|ExecutionSequence`
        (:`then_0`
          ;[1 1 1] Body
          (switch `/Game/YI_ModularZombies/Blueprints/ZombieF02/Demo_Blueprints/ZombieShowcase/Enums/E_ZombieMaterialVariations` (`self.Select Zombie Base Material`)
            (:`NewEnumerator0`
              (`PrimitiveComponent.SetMaterialByName` _sk_zombiefemale02_2 "Body" "/Game/YI_ModularZombies/Materials/ZombieF02/Body/01NoGore/MI_Body_Zombie_F02_01.MI_Body_Zombie_F02_01"))
            (:`NewEnumerator6`
              (`PrimitiveComponent.SetMaterialByName` _sk_zombiefemale02_2 "Body" "/Game/YI_ModularZombies/Materials/ZombieF02/Body/02FullGore/MI_Body_Zombie_F02_02.MI_Body_Zombie_F02_02"))
            (:`NewEnumerator7`
              (`PrimitiveComponent.SetMaterialByName` _sk_zombiefemale02_2 "Body" "/Game/YI_ModularZombies/Materials/ZombieF02/Body/03FullGoreNoHands/MI_Body_Zombie_F02_03.MI_Body_Zombie_F02_03"))
            (:`NewEnumerator8`
              (`PrimitiveComponent.SetMaterialByName` _sk_zombiefemale02_2 "Body" "/Game/YI_ModularZombies/Materials/ZombieF02/Body/04HandsOnly/MI_Body_Zombie_F02_04.MI_Body_Zombie_F02_04"))
            (:`NewEnumerator11`
              (`PrimitiveComponent.SetMaterialByName` _sk_zombiefemale02_2 "Body" "/Game/YI_ModularZombies/Materials/ZombieF02/Body/05WoundOnly/MI_Body_Zombie_F02_05.MI_Body_Zombie_F02_05"))
            (:`NewEnumerator12`
              (`PrimitiveComponent.SetMaterialByName` _sk_zombiefemale02_2 "Body" "/Game/YI_ModularZombies/Materials/ZombieF02/Body/06ChestDripOnly/MI_Body_Zombie_F02_06.MI_Body_Zombie_F02_06"))
            (:`NewEnumerator13`
              (`PrimitiveComponent.SetMaterialByName` _sk_zombiefemale02_2 "Body" "/Game/YI_ModularZombies/Materials/ZombieF02/Body/07WoundHands/MI_Body_Zombie_F02_07.MI_Body_Zombie_F02_07"))
            (:`NewEnumerator14`
              (`PrimitiveComponent.SetMaterialByName` _sk_zombiefemale02_2 "Body" "/Game/YI_ModularZombies/Materials/ZombieF02/Body/08ChestDripHands/MI_Body_Zombie_F02_08.MI_Body_Zombie_F02_08"))))
        (:`then_1`
          ;[1 1 1] HeadVariations
          (switch `/Game/YI_ModularZombies/Blueprints/ZombieF02/Demo_Blueprints/ZombieShowcase/Enums/E_ZombieHeadVariations` (`self.Select Zombie Head Base Material`)
            (:`NewEnumerator0`
              (switch `/Game/YI_ModularZombies/Blueprints/ZombieF02/Demo_Blueprints/ZombieShowcase/Enums/E_ZombieType` _selectzombie
                (:`NewEnumerator0`
                  (`PrimitiveComponent.SetMaterialByName` _sk_zombiefemale02_3 "Head" "/Game/YI_ModularZombies/Materials/ZombieF02/Head01/01NoGore/MI_Head01_Zombie_F02_01.MI_Head01_Zombie_F02_01"))
                (:`NewEnumerator1`
                  (`PrimitiveComponent.SetMaterialByName` _sk_zombiefemale02_3 "Head" "/Game/YI_ModularZombies/Materials/ZombieF02/Head02/01NoGore/MI_Head02_Zombie_F02_01.MI_Head02_Zombie_F02_01"))))
            (:`NewEnumerator6`
              (switch `/Game/YI_ModularZombies/Blueprints/ZombieF02/Demo_Blueprints/ZombieShowcase/Enums/E_ZombieType` _selectzombie
                (:`NewEnumerator0`
                  (`PrimitiveComponent.SetMaterialByName` _sk_zombiefemale02_3 "Head" "/Game/YI_ModularZombies/Materials/ZombieF02/Head01/02FullGore/MI_Head01_Zombie_F02_02.MI_Head01_Zombie_F02_02"))
                (:`NewEnumerator1`
                  (`PrimitiveComponent.SetMaterialByName` _sk_zombiefemale02_3 "Head" "/Game/YI_ModularZombies/Materials/ZombieF02/Head02/02FullGore/MI_Head02_Zombie_F02_02.MI_Head02_Zombie_F02_02"))))
            (:`NewEnumerator7`
              (switch `/Game/YI_ModularZombies/Blueprints/ZombieF02/Demo_Blueprints/ZombieShowcase/Enums/E_ZombieType` _selectzombie
                (:`NewEnumerator0`
                  (`PrimitiveComponent.SetMaterialByName` _sk_zombiefemale02_3 "Head" "/Game/YI_ModularZombies/Materials/ZombieF02/Head01/03LightGore/MI_Head01_Zombie_F02_03.MI_Head01_Zombie_F02_03"))
                (:`NewEnumerator1`
                  (`PrimitiveComponent.SetMaterialByName` _sk_zombiefemale02_3 "Head" "/Game/YI_ModularZombies/Materials/ZombieF02/Head02/03LightGore/MI_Head02_Zombie_F02_03.MI_Head02_Zombie_F02_03"))))
            (:`NewEnumerator8`
              (switch `/Game/YI_ModularZombies/Blueprints/ZombieF02/Demo_Blueprints/ZombieShowcase/Enums/E_ZombieType` _selectzombie
                (:`NewEnumerator0`
                  (`PrimitiveComponent.SetMaterialByName` _sk_zombiefemale02_3 "Head" "/Game/YI_ModularZombies/Materials/ZombieF02/Head01/04MouthGore/MI_Head01_Zombie_F02_04.MI_Head01_Zombie_F02_04"))
                (:`NewEnumerator1`
                  (`PrimitiveComponent.SetMaterialByName` _sk_zombiefemale02_3 "Head" "/Game/YI_ModularZombies/Materials/ZombieF02/Head02/04MouthGore/MI_Head02_Zombie_F02_04.MI_Head02_Zombie_F02_04"))))
            (:`NewEnumerator11`
              (switch `/Game/YI_ModularZombies/Blueprints/ZombieF02/Demo_Blueprints/ZombieShowcase/Enums/E_ZombieType` _selectzombie
                (:`NewEnumerator0`
                  (`PrimitiveComponent.SetMaterialByName` _sk_zombiefemale02_3 "Head" "/Game/YI_ModularZombies/Materials/ZombieF02/Head01/05WoundGore/MI_Head01_Zombie_F02_05.MI_Head01_Zombie_F02_05"))
                (:`NewEnumerator1`
                  (`PrimitiveComponent.SetMaterialByName` _sk_zombiefemale02_3 "Head" "/Game/YI_ModularZombies/Materials/ZombieF02/Head02/05WoundGore/MI_Head02_Zombie_F02_05.MI_Head02_Zombie_F02_05"))))))
        (:`then_2`
          ;[1 1 1] LongPants
          (switch `/Game/YI_ModularZombies/Blueprints/ZombieF02/Demo_Blueprints/ZombieShowcase/Enums/E_Clothing_SkirtMaterialVariations` (`self.Select Cheerleader Skirt Material`)
            (:`NewEnumerator0`
              (`PrimitiveComponent.SetMaterial` _sk_cheerleader_skirt_2 0 "/Game/YI_ModularZombies/Materials/ZombieF02/Clothing/OutfitCheerleader/01CleanRed/MI_Clth_CheerleaderOutfit_F02_01.MI_Clth_CheerleaderOutfit_F02_01"))
            (:`NewEnumerator6`
              (`PrimitiveComponent.SetMaterial` _sk_cheerleader_skirt_2 0 "/Game/YI_ModularZombies/Materials/ZombieF02/Clothing/OutfitCheerleader/02CleanBlue/MI_Clth_CheerleaderOutfit_F02_02.MI_Clth_CheerleaderOutfit_F02_02"))
            (:`NewEnumerator7`
              (`PrimitiveComponent.SetMaterial` _sk_cheerleader_skirt_2 0 "/Game/YI_ModularZombies/Materials/ZombieF02/Clothing/OutfitCheerleader/03CleanGreen/MI_Clth_CheerleaderOutfit_F02_03.MI_Clth_CheerleaderOutfit_F02_03"))
            (:`NewEnumerator8`
              (`PrimitiveComponent.SetMaterial` _sk_cheerleader_skirt_2 0 "/Game/YI_ModularZombies/Materials/ZombieF02/Clothing/OutfitCheerleader/04OldRed/MI_Clth_CheerleaderOutfit_F02_04.MI_Clth_CheerleaderOutfit_F02_04"))
            (:`NewEnumerator9`
              (`PrimitiveComponent.SetMaterial` _sk_cheerleader_skirt_2 0 "/Game/YI_ModularZombies/Materials/ZombieF02/Clothing/OutfitCheerleader/05OldBlue/MI_Clth_CheerleaderOutfit_F02_05.MI_Clth_CheerleaderOutfit_F02_05"))
            (:`NewEnumerator10`
              (`PrimitiveComponent.SetMaterial` _sk_cheerleader_skirt_2 0 "/Game/YI_ModularZombies/Materials/ZombieF02/Clothing/OutfitCheerleader/06OldGreen/MI_Clth_CheerleaderOutfit_F02_06.MI_Clth_CheerleaderOutfit_F02_06"))
            (:`NewEnumerator11`
              (`PrimitiveComponent.SetMaterial` _sk_cheerleader_skirt_2 0 "/Game/YI_ModularZombies/Materials/ZombieF02/Clothing/OutfitCheerleader/07DirtyRed/MI_Clth_CheerleaderOutfit_F02_07.MI_Clth_CheerleaderOutfit_F02_07"))
            (:`NewEnumerator12`
              (`PrimitiveComponent.SetMaterial` _sk_cheerleader_skirt_2 0 "/Game/YI_ModularZombies/Materials/ZombieF02/Clothing/OutfitCheerleader/08DirtyBlue/MI_Clth_CheerleaderOutfit_F02_08.MI_Clth_CheerleaderOutfit_F02_08"))
            (:`NewEnumerator13`
              (`PrimitiveComponent.SetMaterial` _sk_cheerleader_skirt_2 0 "/Game/YI_ModularZombies/Materials/ZombieF02/Clothing/OutfitCheerleader/09DirtyGreen/MI_Clth_CheerleaderOutfit_F02_09.MI_Clth_CheerleaderOutfit_F02_09"))
            (:`NewEnumerator14`
              (`PrimitiveComponent.SetMaterial` _sk_cheerleader_skirt_2 0 "/Game/YI_ModularZombies/Materials/ZombieF02/Clothing/OutfitCheerleader/10DirtyGoreRed/MI_Clth_CheerleaderOutfit_F02_10.MI_Clth_CheerleaderOutfit_F02_10"))
            (:`NewEnumerator15`
              (`PrimitiveComponent.SetMaterial` _sk_cheerleader_skirt_2 0 "/Game/YI_ModularZombies/Materials/ZombieF02/Clothing/OutfitCheerleader/11DirtyGoreBlue/MI_Clth_CheerleaderOutfit_F02_11.MI_Clth_CheerleaderOutfit_F02_11"))
            (:`NewEnumerator16`
              (`PrimitiveComponent.SetMaterial` _sk_cheerleader_skirt_2 0 "/Game/YI_ModularZombies/Materials/ZombieF02/Clothing/OutfitCheerleader/12DirtyGoreGreen/MI_Clth_CheerleaderOutfit_F02_12.MI_Clth_CheerleaderOutfit_F02_12"))
            (:`NewEnumerator17`
              (`PrimitiveComponent.SetMaterial` _sk_cheerleader_skirt_2 0 "/Game/YI_ModularZombies/Materials/ZombieF02/Clothing/OutfitCheerleader/13OldRedGore/MI_Clth_CheerleaderOutfit_F02_13.MI_Clth_CheerleaderOutfit_F02_13"))
            (:`NewEnumerator18`
              (`PrimitiveComponent.SetMaterial` _sk_cheerleader_skirt_2 0 "/Game/YI_ModularZombies/Materials/ZombieF02/Clothing/OutfitCheerleader/14OldBlueGore/MI_Clth_CheerleaderOutfit_F02_14.MI_Clth_CheerleaderOutfit_F02_14"))
            (:`NewEnumerator19`
              (`PrimitiveComponent.SetMaterial` _sk_cheerleader_skirt_2 0 "/Game/YI_ModularZombies/Materials/ZombieF02/Clothing/OutfitCheerleader/15OldGreenGore/MI_Clth_CheerleaderOutfit_F02_15.MI_Clth_CheerleaderOutfit_F02_15"))))
        (:`then_3`
          ;[1 1 1] Singlet
          (switch `/Game/YI_ModularZombies/Blueprints/ZombieF02/Demo_Blueprints/ZombieShowcase/Enums/E_Clothing_SingletMaterialVariations` (`self.Select Cheerleader Top Material`)
            (:`NewEnumerator0`
              (`PrimitiveComponent.SetMaterial` _sk_cheerleader_top_2 0 "/Game/YI_ModularZombies/Materials/ZombieF02/Clothing/OutfitCheerleader/01CleanRed/MI_Clth_CheerleaderOutfit_F02_01.MI_Clth_CheerleaderOutfit_F02_01"))
            (:`NewEnumerator6`
              (`PrimitiveComponent.SetMaterial` _sk_cheerleader_top_2 0 "/Game/YI_ModularZombies/Materials/ZombieF02/Clothing/OutfitCheerleader/02CleanBlue/MI_Clth_CheerleaderOutfit_F02_02.MI_Clth_CheerleaderOutfit_F02_02"))
            (:`NewEnumerator7`
              (`PrimitiveComponent.SetMaterial` _sk_cheerleader_top_2 0 "/Game/YI_ModularZombies/Materials/ZombieF02/Clothing/OutfitCheerleader/03CleanGreen/MI_Clth_CheerleaderOutfit_F02_03.MI_Clth_CheerleaderOutfit_F02_03"))
            (:`NewEnumerator8`
              (`PrimitiveComponent.SetMaterial` _sk_cheerleader_top_2 0 "/Game/YI_ModularZombies/Materials/ZombieF02/Clothing/OutfitCheerleader/04OldRed/MI_Clth_CheerleaderOutfit_F02_04.MI_Clth_CheerleaderOutfit_F02_04"))
            (:`NewEnumerator9`
              (`PrimitiveComponent.SetMaterial` _sk_cheerleader_top_2 0 "/Game/YI_ModularZombies/Materials/ZombieF02/Clothing/OutfitCheerleader/05OldBlue/MI_Clth_CheerleaderOutfit_F02_05.MI_Clth_CheerleaderOutfit_F02_05"))
            (:`NewEnumerator10`
              (`PrimitiveComponent.SetMaterial` _sk_cheerleader_top_2 0 "/Game/YI_ModularZombies/Materials/ZombieF02/Clothing/OutfitCheerleader/06OldGreen/MI_Clth_CheerleaderOutfit_F02_06.MI_Clth_CheerleaderOutfit_F02_06"))
            (:`NewEnumerator11`
              (`PrimitiveComponent.SetMaterial` _sk_cheerleader_top_2 0 "/Game/YI_ModularZombies/Materials/ZombieF02/Clothing/OutfitCheerleader/07DirtyRed/MI_Clth_CheerleaderOutfit_F02_07.MI_Clth_CheerleaderOutfit_F02_07"))
            (:`NewEnumerator12`
              (`PrimitiveComponent.SetMaterial` _sk_cheerleader_top_2 0 "/Game/YI_ModularZombies/Materials/ZombieF02/Clothing/OutfitCheerleader/08DirtyBlue/MI_Clth_CheerleaderOutfit_F02_08.MI_Clth_CheerleaderOutfit_F02_08"))
            (:`NewEnumerator13`
              (`PrimitiveComponent.SetMaterial` _sk_cheerleader_top_2 0 "/Game/YI_ModularZombies/Materials/ZombieF02/Clothing/OutfitCheerleader/09DirtyGreen/MI_Clth_CheerleaderOutfit_F02_09.MI_Clth_CheerleaderOutfit_F02_09"))
            (:`NewEnumerator14`
              (`PrimitiveComponent.SetMaterial` _sk_cheerleader_top_2 0 "/Game/YI_ModularZombies/Materials/ZombieF02/Clothing/OutfitCheerleader/10DirtyGoreRed/MI_Clth_CheerleaderOutfit_F02_10.MI_Clth_CheerleaderOutfit_F02_10"))
            (:`NewEnumerator15`
              (`PrimitiveComponent.SetMaterial` _sk_cheerleader_top_2 0 "/Game/YI_ModularZombies/Materials/ZombieF02/Clothing/OutfitCheerleader/11DirtyGoreBlue/MI_Clth_CheerleaderOutfit_F02_11.MI_Clth_CheerleaderOutfit_F02_11"))
            (:`NewEnumerator16`
              (`PrimitiveComponent.SetMaterial` _sk_cheerleader_top_2 0 "/Game/YI_ModularZombies/Materials/ZombieF02/Clothing/OutfitCheerleader/12DirtyGoreGreen/MI_Clth_CheerleaderOutfit_F02_12.MI_Clth_CheerleaderOutfit_F02_12"))
            (:`NewEnumerator17`
              (`PrimitiveComponent.SetMaterial` _sk_cheerleader_top_2 0 "/Game/YI_ModularZombies/Materials/ZombieF02/Clothing/OutfitCheerleader/13OldRedGore/MI_Clth_CheerleaderOutfit_F02_13.MI_Clth_CheerleaderOutfit_F02_13"))
            (:`NewEnumerator18`
              (`PrimitiveComponent.SetMaterial` _sk_cheerleader_top_2 0 "/Game/YI_ModularZombies/Materials/ZombieF02/Clothing/OutfitCheerleader/14OldBlueGore/MI_Clth_CheerleaderOutfit_F02_14.MI_Clth_CheerleaderOutfit_F02_14"))
            (:`NewEnumerator19`
              (`PrimitiveComponent.SetMaterial` _sk_cheerleader_top_2 0 "/Game/YI_ModularZombies/Materials/ZombieF02/Clothing/OutfitCheerleader/15OldGreenGore/MI_Clth_CheerleaderOutfit_F02_15.MI_Clth_CheerleaderOutfit_F02_15"))))
        (:`then_4`
          ;[1 1 1] Tshirt
          (switch `/Game/YI_ModularZombies/Blueprints/ZombieF02/Demo_Blueprints/ZombieShowcase/Enums/E_Clothing_BraLingerieMaterialVariations` (`self.Select Bra Material`)
            (:`NewEnumerator0`
              (`PrimitiveComponent.SetMaterial` _sk_bralingerie_2 0 "/Game/YI_ModularZombies/Materials/ZombieF02/Clothing/OutfitLingerie/BraLingerie/01CleanWhite/MI_Clth_BraLingerie_F02_01.MI_Clth_BraLingerie_F02_01"))
            (:`NewEnumerator6`
              (`PrimitiveComponent.SetMaterial` _sk_bralingerie_2 0 "/Game/YI_ModularZombies/Materials/ZombieF02/Clothing/OutfitLingerie/BraLingerie/02CleanRed/MI_Clth_BraLingerie_F02_02.MI_Clth_BraLingerie_F02_02"))
            (:`NewEnumerator7`
              (`PrimitiveComponent.SetMaterial` _sk_bralingerie_2 0 "/Game/YI_ModularZombies/Materials/ZombieF02/Clothing/OutfitLingerie/BraLingerie/03DirtyWhite/MI_Clth_BraLingerie_F02_03.MI_Clth_BraLingerie_F02_03"))
            (:`NewEnumerator8`
              (`PrimitiveComponent.SetMaterial` _sk_bralingerie_2 0 "/Game/YI_ModularZombies/Materials/ZombieF02/Clothing/OutfitLingerie/BraLingerie/04DirtyRed/MI_Clth_BraLingerie_F02_04.MI_Clth_BraLingerie_F02_04"))
            (:`NewEnumerator9`
              (`PrimitiveComponent.SetMaterial` _sk_bralingerie_2 0 "/Game/YI_ModularZombies/Materials/ZombieF02/Clothing/OutfitLingerie/BraLingerie/05DirtyBlack/MI_Clth_BraLingerie_F02_05.MI_Clth_BraLingerie_F02_05"))
            (:`NewEnumerator10`
              (`PrimitiveComponent.SetMaterial` _sk_bralingerie_2 0 "/Game/YI_ModularZombies/Materials/ZombieF02/Clothing/OutfitLingerie/BraLingerie/06DirtyGoreWhite/MI_Clth_BraLingerie_F02_06.MI_Clth_BraLingerie_F02_06"))
            (:`NewEnumerator11`
              (`PrimitiveComponent.SetMaterial` _sk_bralingerie_2 0 "/Game/YI_ModularZombies/Materials/ZombieF02/Clothing/OutfitLingerie/BraLingerie/07DirtyGoreRed/MI_Clth_BraLingerie_F02_07.MI_Clth_BraLingerie_F02_07"))
            (:`NewEnumerator12`
              (`PrimitiveComponent.SetMaterial` _sk_bralingerie_2 0 "/Game/YI_ModularZombies/Materials/ZombieF02/Clothing/OutfitLingerie/BraLingerie/08DirtyGoreBlack/MI_Clth_BraLingerie_F02_08.MI_Clth_BraLingerie_F02_08"))))
        (:`then_5`
          ;[1 1 1] Hair Color
          (switch `/Game/YI_ModularZombies/Blueprints/ZombieF02/Demo_Blueprints/ZombieShowcase/Enums/E_HairColorsMaterialVariations` (`self.Select Hair Color`)
            (:`NewEnumerator0`
              (`PrimitiveComponent.SetMaterialByName` _sk_hair_2 "Hair" "/Game/YI_ModularZombies/Materials/ZombieF02/Hair/01Blonde/MI_Hair_F02_01.MI_Hair_F02_01")
              (`PrimitiveComponent.SetMaterialByName` _sk_hair_2 "HairCap" "/Game/YI_ModularZombies/Materials/ZombieF02/Hair/01Blonde/MI_Haircap_F02_01.MI_Haircap_F02_01"))
            (:`NewEnumerator4`
              (`PrimitiveComponent.SetMaterialByName` _sk_hair_2 "Hair" "/Game/YI_ModularZombies/Materials/ZombieF02/Hair/02BlondeDirty/MI_Hair_F02_02.MI_Hair_F02_02")
              (`PrimitiveComponent.SetMaterialByName` _sk_hair_2 "HairCap" "/Game/YI_ModularZombies/Materials/ZombieF02/Hair/02BlondeDirty/MI_Haircap_F02_02.MI_Haircap_F02_02"))))))
    (:`then_2`
      ;[1 1 1] Showcase Light Settings
      (if (`self.ShowcaseLightsOn?`)
        (`SceneComponent.SetVisibility` (`self.RotatingLight_01`) true false)
        (`SceneComponent.SetVisibility` (`self.RotatingLight_02`) true false)
        (if (`self.ShowcaseLightsShadows?`)
          (`LightComponentBase.SetCastShadows` (`self.RotatingLight_01`) true)
          (`LightComponentBase.SetCastShadows` (`self.RotatingLight_02`) true)
          (else
            (`LightComponentBase.SetCastShadows` (`self.RotatingLight_02`) false)
            (`LightComponentBase.SetCastShadows` (`self.RotatingLight_01`) false)))
        (else
          (`SceneComponent.SetVisibility` (`self.RotatingLight_02`) false false)
          (`SceneComponent.SetVisibility` (`self.RotatingLight_01`) false false)
          (set `self.ShowcaseLightsRotate?` false))))))