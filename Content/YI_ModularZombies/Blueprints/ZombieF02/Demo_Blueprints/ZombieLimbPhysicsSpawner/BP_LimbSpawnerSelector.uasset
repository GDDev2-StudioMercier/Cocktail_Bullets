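; Limb actor from the modular zombie demo that shows a randomly chosen skeletal mesh from LimbsToSpawn on its SKLimb component.
; On BeginPlay, it enables physics simulation below each listed bone if SKLimb's display name contains "torso", a check made before the random mesh is assigned.
; Tick runs a Delay and then destroys the actor when DestroyTime is above zero.
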(event `self.ReceiveBeginPlay`
  (bind _limbstospawn (`self.LimbsToSpawn`))
  (if (`KismetStringLibrary.Contains` (`KismetSystemLibrary.GetDisplayName` (`self.SK_Limb`)) "torso")
    (for _array_element (`self.BoneNames`)
      (`SkeletalMeshComponent.SetAllBodiesBelowSimulatePhysics` (`self.SK_Limb`) _array_element true true)))
  (`SkinnedMeshComponent.SetSkinnedAssetAndUpdate` (`self.SK_Limb`) (`|GetArrayItem` _limbstospawn (`KismetMathLibrary.RandomInteger` (`KismetArrayLibrary.Array_Length` _limbstospawn))) true))

(event `self.ReceiveTick`
  (params (DeltaSeconds :type "Float (single-precision)"))
  (bind _destroytime (`self.DestroyTime`))
  (if (> _destroytime 0.0)
    (`KismetSystemLibrary.Delay` _destroytime)
    (`self.K2_DestroyActor`)))

(fn `UserConstructionScript`)