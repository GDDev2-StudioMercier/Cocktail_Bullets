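; BP_DismemberedLimb is an actor for a severed zombie limb, with optional timed cleanup.
; On BeginPlay, SetBonePhysics loops over BoneNames and, only when TargetLimb's display name contains "torso", enables physics simulation on bodies below each bone, excluding that bone.
; Tick destroys the actor through a Delay whenever Timer is above zero.
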(event `self.ReceiveBeginPlay`
  (`self.SetBonePhysics`))

(event `self.ReceiveTick`
  (params (DeltaSeconds :type "Float (single-precision)"))
  (bind _timer (`self.Timer`))
  (if (> _timer 0.0)
    (`KismetSystemLibrary.Delay` _timer)
    (`self.K2_DestroyActor`)))

(fn `SetBonePhysics`
  (bind _targetlimb (`self.TargetLimb`))
  (for _array_element (`self.BoneNames`)
    (if (`KismetStringLibrary.Contains` (`KismetSystemLibrary.GetDisplayName` _targetlimb) "torso")
      (`SkeletalMeshComponent.SetAllBodiesBelowSimulatePhysics` _targetlimb _array_element true false))))

(fn `UserConstructionScript`)