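; Demo zombie actor that repeatedly blows apart into physics-driven limbs and reappears, showcasing dismemberment.
; The construction script makes the arm, leg and torso meshes follow the head mesh's pose as leader component.
; Tick runs a Delay-paced cycle that toggles the head mesh's visibility, propagated to children, around each Explode call.
; Explode spawns the listed limb classes at the actor's location, passes on a Timer and launches each with a random upward impulse.
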(event `self.ReceiveTick`
  (params (DeltaSeconds :type "Float (single-precision)"))
  (`KismetSystemLibrary.Delay` 1.0)
  (`self.ToggleVisibilityZombie`)
  (`self.Explode`)
  (`KismetSystemLibrary.Delay` 0.5)
  (`self.ToggleVisibilityZombie`)
  (`KismetSystemLibrary.Delay` 1.0))

(fn `Explode`
  (bind _returnvalue (`KismetMathLibrary.RandomFloatInRange` -250.0 250.0))
  (for _array_element (`self.LimbToSpawnList`)
    (bind _returnvalue_2 (`|SpawnActorFromClass` _array_element (`KismetMathLibrary.Conv_VectorToTransform` (`self.K2_GetActorLocation`)) "Undefined" "SelectDefaultAtRuntime" null 0.0 null))
    (bind _asbp_dismembered_limb (cast `/Game/YI_ModularZombies/Blueprints/ZombieM01/Demo_Blueprints/ZombieExplode/Limbs/BP_DismemberedLimb` _returnvalue_2))
    (set `/Game/YI_ModularZombies/Blueprints/ZombieM01/Demo_Blueprints/ZombieExplode/Limbs/BP_DismemberedLimb.Timer` (`self.Timer`) _asbp_dismembered_limb)
    (bind _targetlimb (`/Game/YI_ModularZombies/Blueprints/ZombieM01/Demo_Blueprints/ZombieExplode/Limbs/BP_DismemberedLimb.TargetLimb` _asbp_dismembered_limb))
    (`PrimitiveComponent.SetCollisionEnabled` _targetlimb "PhysicsOnly")
    (`PrimitiveComponent.SetSimulatePhysics` _targetlimb true)
    (`PrimitiveComponent.AddImpulse` _targetlimb (`KismetMathLibrary.MakeVector` _returnvalue _returnvalue (`KismetMathLibrary.RandomFloatInRange` 500.0 750.0)) "None" true)))

(fn `ToggleVisibilityZombie`
  (`SceneComponent.ToggleVisibility` (`self.SK_ZombieLimb_Head01`) true))

(fn `UserConstructionScript`
  (`SkinnedMeshComponent.SetLeaderPoseComponent` (`self.SK_ZombieLimb_LeftArm`) (`self.SK_ZombieLimb_Head01`) false false)
  (`SkinnedMeshComponent.SetLeaderPoseComponent` (`self.SK_ZombieLimb_LeftLeg`) (`self.SK_ZombieLimb_Head01`) false false)
  (`SkinnedMeshComponent.SetLeaderPoseComponent` (`self.SK_ZombieLimb_RightArm`) (`self.SK_ZombieLimb_Head01`) false false)
  (`SkinnedMeshComponent.SetLeaderPoseComponent` (`self.SK_ZombieLimb_RightLeg`) (`self.SK_ZombieLimb_Head01`) false false)
  (`SkinnedMeshComponent.SetLeaderPoseComponent` (`self.SK_ZombieLimb_TorsoHead01`) (`self.SK_ZombieLimb_Head01`) false false))