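; Demo showcase actor that previews outfit and material combinations for the modular male M01 zombie.
; The Construction Script applies selection variables: it swaps the zombie mesh, offsets the beanie per head, toggles clothing visibility and assigns materials.
; It also sets visibility and shadows on two showcase lights, disabling rotation when they are off.
; While rotation is enabled, Tick yaws the Box component in steps throttled by a Delay.
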(event `self.ReceiveTick`
  (params (DeltaSeconds :type "Float (single-precision)"))
  (bind _box (`self.Box`))
  (bind (_returnvalue_roll _returnvalue_pitch _returnvalue_yaw) (`KismetMathLibrary.BreakRotator` (`SceneComponent.K2_GetComponentRotation` _box)))
  (if (`self.ShowcaseLightsRotate?`)
    (`KismetSystemLibrary.Delay` (`self.RotationTickDelay`))
    (`SceneComponent.K2_SetWorldRotation` _box (`KismetMathLibrary.MakeRotator` _returnvalue_roll _returnvalue_pitch (+ _returnvalue_yaw (`self.RotationPerTick`))) false false)))

(fn `UserConstructionScript`
  (bind _sk_zombiemale01 (`self.SK_ZombieMale01`))
  (bind _sk_zombiemale01_2 (`self.SK_ZombieMale01`))
  (bind _sk_zombiemale01_3 (`self.SK_ZombieMale01`))
  (bind _sk_zombiemale01_4 (`self.SK_ZombieMale01`))
  (bind _sk_zombiemale01_5 (`self.SK_ZombieMale01`))
  (bind _sm_clothing_beanie (`self.SM_Clothing_Beanie`))
  (bind _sk_clothing_poloshirt (`self.SK_Clothing_PoloShirt`))
  (bind _sk_clothing_singlet (`self.SK_Clothing_Singlet`))
  (bind _sm_clothing_beanie_2 (`self.SM_Clothing_Beanie`))
  (bind _sk_zombiemale01_6 (`self.SK_ZombieMale01`))
  (bind _sm_clothing_beanie_3 (`self.SM_Clothing_Beanie`))
  (bind _sk_clothing_singlet_2 (`self.SK_Clothing_Singlet`))
  (bind _sk_clothing_poloshirt_2 (`self.SK_Clothing_PoloShirt`))
  (bind _sk_clothing_shorts (`self.SK_Clothing_Shorts`))
  (bind _sm_clothing_beanie_4 (`self.SM_Clothing_Beanie`))
  (bind _sk_zombiemale01_7 (`self.SK_ZombieMale01`))
  (bind _sk_clothing_shorts_2 (`self.SK_Clothing_Shorts`))
  (bind _sk_zombiemale01_8 (`self.SK_ZombieMale01`))
  (bind _sk_zombiemale01_9 (`self.SK_ZombieMale01`))
  (bind _sk_zombiemale01_10 (`self.SK_ZombieMale01`))
  (bind _sk_zombiemale01_11 (`self.SK_ZombieMale01`))
  (bind _returnvalue_location (`KismetMathLibrary.BreakTransform` (`SceneComponent.GetSocketTransform` _sm_clothing_beanie_2 "None" "RTS_World")))
  (bind _returnvalue_location_2 (`KismetMathLibrary.BreakTransform` (`SceneComponent.GetSocketTransform` _sm_clothing_beanie_4 "None" "RTS_World")))
  (`|ExecutionSequence`
    (:`then_0`
      ;[1 1 1] Select Mesh Options
      (`|ExecutionSequence`
        (:`then_0`
          (switch `/Game/YI_ModularZombies/Blueprints/ZombieM01/Demo_Blueprints/ZombieShowcase/Enums/E_PantsType` (`self.SelectPants`)
            (:`NewEnumerator0`
              (`SceneComponent.SetVisibility` _sk_clothing_shorts_2 false false))
            (:`NewEnumerator1`
              (`SceneComponent.SetVisibility` _sk_clothing_shorts_2 true false))))
        (:`then_1`
          (switch `/Game/YI_ModularZombies/Blueprints/ZombieM01/Demo_Blueprints/ZombieShowcase/Enums/E_ShirtType` (`self.SelectShirt`)
            (:`NewEnumerator0`
              (`SceneComponent.SetVisibility` _sk_clothing_poloshirt false false)
              (`SceneComponent.SetVisibility` _sk_clothing_singlet false false))
            (:`NewEnumerator1`
              (`SceneComponent.SetVisibility` _sk_clothing_poloshirt true false)
              (`SceneComponent.SetVisibility` _sk_clothing_singlet false false))
            (:`NewEnumerator2`
              (`SceneComponent.SetVisibility` _sk_clothing_singlet true false)
              (`SceneComponent.SetVisibility` _sk_clothing_poloshirt false false))))
        (:`then_2`
          (switch `/Game/YI_ModularZombies/Blueprints/ZombieM01/Demo_Blueprints/ZombieShowcase/Enums/E_ZombieType` (`self.SelectZombie`)
            (:`NewEnumerator0`
              (`SkinnedMeshComponent.SetSkinnedAssetAndUpdate` _sk_zombiemale01 "/Game/YI_ModularZombies/Meshes/ZombieM01/Zombie/SK_Zombie_M01_01.SK_Zombie_M01_01" true)
              (`SceneComponent.K2_SetWorldTransform` _sm_clothing_beanie_4 (`KismetMathLibrary.MakeTransform` (- _returnvalue_location_2 (`self.BeanieLocationHead01`))) false false))
            (:`NewEnumerator1`
              (`SkinnedMeshComponent.SetSkinnedAssetAndUpdate` _sk_zombiemale01 "/Game/YI_ModularZombies/Meshes/ZombieM01/Zombie/SK_Zombie_M01_02.SK_Zombie_M01_02" true)
              (`SceneComponent.K2_SetWorldTransform` _sm_clothing_beanie_2 (`KismetMathLibrary.MakeTransform` (- _returnvalue_location (`self.BeanieLocationHead02`))) false false))))
        (:`then_3`
          (switch `/Game/YI_ModularZombies/Blueprints/ZombieM01/Demo_Blueprints/ZombieShowcase/Enums/E_HeadAccessoryType` (`self.SelectHeadAccessory`)
            (:`NewEnumerator0`
              (`SceneComponent.SetVisibility` _sm_clothing_beanie false false))
            (:`NewEnumerator1`
              (`SceneComponent.SetVisibility` _sm_clothing_beanie true false))))))
    (:`then_1`
      (`|ExecutionSequence`
        (:`then_0`
          (switch `/Game/YI_ModularZombies/Blueprints/ZombieM01/Demo_Blueprints/ZombieShowcase/Enums/E_ZombieType` (`self.SelectZombie`)
            (:`NewEnumerator0`
              (switch `/Game/YI_ModularZombies/Blueprints/ZombieM01/Demo_Blueprints/ZombieShowcase/Enums/E_ZombieMaterialVariations` (`self.Select Zombie Base Material`)
                (:`NewEnumerator0`
                  (`PrimitiveComponent.SetMaterialByName` _sk_zombiemale01_11 "Body" "/Game/YI_ModularZombies/Materials/ZombieM01/Body/01Skin01Default/MI_Body_Zombie_M01_01.MI_Body_Zombie_M01_01")
                  (`PrimitiveComponent.SetMaterialByName` _sk_zombiemale01_11 "Head" "/Game/YI_ModularZombies/Materials/ZombieM01/Head01/01Skin01Default/MI_Head01_M01_01.MI_Head01_M01_01"))
                (:`NewEnumerator1`
                  (`PrimitiveComponent.SetMaterialByName` _sk_zombiemale01_2 "Body" "/Game/YI_ModularZombies/Materials/ZombieM01/Body/02Skin02Decayed/MI_Body_Zombie_M01_02.MI_Body_Zombie_M01_02")
                  (`PrimitiveComponent.SetMaterialByName` _sk_zombiemale01_2 "Head" "/Game/YI_ModularZombies/Materials/ZombieM01/Head01/02Skin02Decayed/MI_Head01_M01_02.MI_Head01_M01_02"))
                (:`NewEnumerator2`
                  (`PrimitiveComponent.SetMaterialByName` _sk_zombiemale01_3 "Body" "/Game/YI_ModularZombies/Materials/ZombieM01/Body/03Skin03Burnt/MI_Body_Zombie_M01_03.MI_Body_Zombie_M01_03")
                  (`PrimitiveComponent.SetMaterialByName` _sk_zombiemale01_3 "Head" "/Game/YI_ModularZombies/Materials/ZombieM01/Head01/03Skin03Burnt/MI_Head01_M01_03.MI_Head01_M01_03"))
                (:`NewEnumerator3`
                  (`PrimitiveComponent.SetMaterialByName` _sk_zombiemale01_4 "Body" "/Game/YI_ModularZombies/Materials/ZombieM01/Body/04Skin01NoGore/MI_Body_Zombie_M01_04.MI_Body_Zombie_M01_04")
                  (`PrimitiveComponent.SetMaterialByName` _sk_zombiemale01_4 "Head" "/Game/YI_ModularZombies/Materials/ZombieM01/Head01/01Skin01Default/MI_Head01_M01_01.MI_Head01_M01_01"))
                (:`NewEnumerator5`
                  (`PrimitiveComponent.SetMaterialByName` _sk_zombiemale01_5 "Body" "/Game/YI_ModularZombies/Materials/ZombieM01/Body/05Skin02NoGore/MI_Body_Zombie_M01_05.MI_Body_Zombie_M01_05")
                  (`PrimitiveComponent.SetMaterialByName` _sk_zombiemale01_5 "Head" "/Game/YI_ModularZombies/Materials/ZombieM01/Head01/02Skin02Decayed/MI_Head01_M01_02.MI_Head01_M01_02"))))
            (:`NewEnumerator1`
              (switch `/Game/YI_ModularZombies/Blueprints/ZombieM01/Demo_Blueprints/ZombieShowcase/Enums/E_ZombieMaterialVariations` (`self.Select Zombie Base Material`)
                (:`NewEnumerator0`
                  (`PrimitiveComponent.SetMaterialByName` _sk_zombiemale01_7 "Body" "/Game/YI_ModularZombies/Materials/ZombieM01/Body/01Skin01Default/MI_Body_Zombie_M01_01.MI_Body_Zombie_M01_01")
                  (`PrimitiveComponent.SetMaterialByName` _sk_zombiemale01_7 "Head" "/Game/YI_ModularZombies/Materials/ZombieM01/Head02/01Skin01Default/MI_Head02_M01_01.MI_Head02_M01_01"))
                (:`NewEnumerator1`
                  (`PrimitiveComponent.SetMaterialByName` _sk_zombiemale01_8 "Body" "/Game/YI_ModularZombies/Materials/ZombieM01/Body/02Skin02Decayed/MI_Body_Zombie_M01_02.MI_Body_Zombie_M01_02")
                  (`PrimitiveComponent.SetMaterialByName` _sk_zombiemale01_8 "Head" "/Game/YI_ModularZombies/Materials/ZombieM01/Head02/02Skin02Decayed/MI_Head02_M01_02.MI_Head02_M01_02"))
                (:`NewEnumerator2`
                  (`PrimitiveComponent.SetMaterialByName` _sk_zombiemale01_9 "Body" "/Game/YI_ModularZombies/Materials/ZombieM01/Body/03Skin03Burnt/MI_Body_Zombie_M01_03.MI_Body_Zombie_M01_03")
                  (`PrimitiveComponent.SetMaterialByName` _sk_zombiemale01_9 "Head" "/Game/YI_ModularZombies/Materials/ZombieM01/Head02/03Skin03Burnt/MI_Head02_M01_03.MI_Head02_M01_03"))
                (:`NewEnumerator3`
                  (`PrimitiveComponent.SetMaterialByName` _sk_zombiemale01_10 "Body" "/Game/YI_ModularZombies/Materials/ZombieM01/Body/04Skin01NoGore/MI_Body_Zombie_M01_04.MI_Body_Zombie_M01_04")
                  (`PrimitiveComponent.SetMaterialByName` _sk_zombiemale01_10 "Head" "/Game/YI_ModularZombies/Materials/ZombieM01/Head02/01Skin01Default/MI_Head02_M01_01.MI_Head02_M01_01"))
                (:`NewEnumerator5`
                  (`PrimitiveComponent.SetMaterialByName` _sk_zombiemale01_6 "Body" "/Game/YI_ModularZombies/Materials/ZombieM01/Body/05Skin02NoGore/MI_Body_Zombie_M01_05.MI_Body_Zombie_M01_05")
                  (`PrimitiveComponent.SetMaterialByName` _sk_zombiemale01_6 "Head" "/Game/YI_ModularZombies/Materials/ZombieM01/Head02/02Skin02Decayed/MI_Head02_M01_02.MI_Head02_M01_02"))))))
        (:`then_1`
          (switch `/Game/YI_ModularZombies/Blueprints/ZombieM01/Demo_Blueprints/ZombieShowcase/Enums/E_Clothing_BeanieMaterialVariations` (`self.Select Beanie Material`)
            (:`NewEnumerator0`
              (`PrimitiveComponent.SetMaterial` _sm_clothing_beanie_3 0 "/Game/YI_ModularZombies/Materials/ZombieM01/Clothing/Beanie/01BlackGore/MI_Clth_Beanie_M01_01.MI_Clth_Beanie_M01_01"))
            (:`NewEnumerator1`
              (`PrimitiveComponent.SetMaterial` _sm_clothing_beanie_3 0 "/Game/YI_ModularZombies/Materials/ZombieM01/Clothing/Beanie/02PurpleYellow/MI_Clth_Beanie_M01_02.MI_Clth_Beanie_M01_02"))
            (:`NewEnumerator2`
              (`PrimitiveComponent.SetMaterial` _sm_clothing_beanie_3 0 "/Game/YI_ModularZombies/Materials/ZombieM01/Clothing/Beanie/03GrayGore/MI_Clth_Beanie_M01_03.MI_Clth_Beanie_M01_03"))
            (:`NewEnumerator3`
              (`PrimitiveComponent.SetMaterial` _sm_clothing_beanie_3 0 "/Game/YI_ModularZombies/Materials/ZombieM01/Clothing/Beanie/04OrangeGore/MI_Clth_Beanie_M01_04.MI_Clth_Beanie_M01_04"))
            (:`NewEnumerator5`
              (`PrimitiveComponent.SetMaterial` _sm_clothing_beanie_3 0 "/Game/YI_ModularZombies/Materials/ZombieM01/Clothing/Beanie/05WhiteNoGore/MI_Clth_Beanie_M01_NoGore_05.MI_Clth_Beanie_M01_NoGore_05"))))
        (:`then_2`
          (switch `/Game/YI_ModularZombies/Blueprints/ZombieM01/Demo_Blueprints/ZombieShowcase/Enums/E_Clothing_SingletMaterialVariations` (`self.Select Singlet Material`)
            (:`NewEnumerator0`
              (`PrimitiveComponent.SetMaterial` _sk_clothing_singlet_2 0 "/Game/YI_ModularZombies/Materials/ZombieM01/Clothing/Singlet/01BeaterBlue/MI_Clth_Singlet_M01_01.MI_Clth_Singlet_M01_01"))
            (:`NewEnumerator1`
              (`PrimitiveComponent.SetMaterial` _sk_clothing_singlet_2 0 "/Game/YI_ModularZombies/Materials/ZombieM01/Clothing/Singlet/02BeaterSafety/MI_Clth_Singlet_M01_02.MI_Clth_Singlet_M01_02"))
            (:`NewEnumerator2`
              (`PrimitiveComponent.SetMaterial` _sk_clothing_singlet_2 0 "/Game/YI_ModularZombies/Materials/ZombieM01/Clothing/Singlet/03BeaterWhite/MI_Clth_Singlet_M01_03.MI_Clth_Singlet_M01_03"))
            (:`NewEnumerator3`
              (`PrimitiveComponent.SetMaterial` _sk_clothing_singlet_2 0 "/Game/YI_ModularZombies/Materials/ZombieM01/Clothing/Singlet/04StylishBlue/MI_Clth_Singlet_M01_04.MI_Clth_Singlet_M01_04"))
            (:`NewEnumerator5`
              (`PrimitiveComponent.SetMaterial` _sk_clothing_singlet_2 0 "/Game/YI_ModularZombies/Materials/ZombieM01/Clothing/Singlet/05WhiteNoGore/MI_Clth_Singlet_M01_NoGore_05.MI_Clth_Singlet_M01_NoGore_05"))))
        (:`then_3`
          (switch `/Game/YI_ModularZombies/Blueprints/ZombieM01/Demo_Blueprints/ZombieShowcase/Enums/E_Clothing_PoloShirtMaterialVariations` (`self.Select Poloshirt Material`)
            (:`NewEnumerator0`
              (`PrimitiveComponent.SetMaterial` _sk_clothing_poloshirt_2 0 "/Game/YI_ModularZombies/Materials/ZombieM01/Clothing/Poloshirt/01WhiteGore/MI_Clth_PoloShirt_M01_01.MI_Clth_PoloShirt_M01_01"))
            (:`NewEnumerator1`
              (`PrimitiveComponent.SetMaterial` _sk_clothing_poloshirt_2 0 "/Game/YI_ModularZombies/Materials/ZombieM01/Clothing/Poloshirt/02RedGreenGore/MI_Clth_PoloShirt_M01_02.MI_Clth_PoloShirt_M01_02"))
            (:`NewEnumerator2`
              (`PrimitiveComponent.SetMaterial` _sk_clothing_poloshirt_2 0 "/Game/YI_ModularZombies/Materials/ZombieM01/Clothing/Poloshirt/03WhiteBlueGore/MI_Clth_PoloShirt_M01_03.MI_Clth_PoloShirt_M01_03"))
            (:`NewEnumerator3`
              (`PrimitiveComponent.SetMaterial` _sk_clothing_poloshirt_2 0 "/Game/YI_ModularZombies/Materials/ZombieM01/Clothing/Poloshirt/04WhiteBlackStripedNoGore/MI_Clth_PoloShirt_M01_NoGore_04.MI_Clth_PoloShirt_M01_NoGore_04"))
            (:`NewEnumerator5`
              (`PrimitiveComponent.SetMaterial` _sk_clothing_poloshirt_2 0 "/Game/YI_ModularZombies/Materials/ZombieM01/Clothing/Poloshirt/05WhiteNoGore/MI_Clth_PoloShirt_M01_NoGore_05.MI_Clth_PoloShirt_M01_NoGore_05"))))
        (:`then_4`
          (switch `/Game/YI_ModularZombies/Blueprints/ZombieM01/Demo_Blueprints/ZombieShowcase/Enums/E_Clothing_DenimShortsMaterialVariations` (`self.Select Denim Pants Material`)
            (:`NewEnumerator0`
              (`PrimitiveComponent.SetMaterial` _sk_clothing_shorts 0 "/Game/YI_ModularZombies/Materials/ZombieM01/Clothing/Shorts/01BlueDenim/MI_Clth_Shorts_M01_01.MI_Clth_Shorts_M01_01"))
            (:`NewEnumerator1`
              (`PrimitiveComponent.SetMaterial` _sk_clothing_shorts 0 "/Game/YI_ModularZombies/Materials/ZombieM01/Clothing/Shorts/02Khaki/MI_Clth_Shorts_M01_02.MI_Clth_Shorts_M01_02"))
            (:`NewEnumerator2`
              (`PrimitiveComponent.SetMaterial` _sk_clothing_shorts 0 "/Game/YI_ModularZombies/Materials/ZombieM01/Clothing/Shorts/03Camo/MI_Clth_Shorts_M01_03.MI_Clth_Shorts_M01_03"))
            (:`NewEnumerator3`
              (`PrimitiveComponent.SetMaterial` _sk_clothing_shorts 0 "/Game/YI_ModularZombies/Materials/ZombieM01/Clothing/Shorts/04BlackDenim/MI_Clth_Shorts_M01_04.MI_Clth_Shorts_M01_04"))
            (:`NewEnumerator5`
              (`PrimitiveComponent.SetMaterial` _sk_clothing_shorts 0 "/Game/YI_ModularZombies/Materials/ZombieM01/Clothing/Shorts/05BlueNoGore/MI_Clth_Shorts_M01_NoGore_05.MI_Clth_Shorts_M01_NoGore_05"))
            (:`NewEnumerator6`
              (`PrimitiveComponent.SetMaterial` _sk_clothing_shorts 0 "/Game/YI_ModularZombies/Materials/ZombieM01/Clothing/Shorts/06WhiteNoGore/MI_Clth_Shorts_M01_NoGore_06.MI_Clth_Shorts_M01_NoGore_06"))))))
    (:`then_2`
      (if (`self.ShowcaseLightsOn?`)
        (`SceneComponent.SetVisibility` (`self.RotatingLight_01`) true false)
        (`SceneComponent.SetVisibility` (`self.RotatingLight_02`) true false)
        (if (`self.ShowcaseLightsShadows?`)
          (`LightComponentBase.SetCastShadows` (`self.RotatingLight_01`) true)
          (`LightComponentBase.SetCastShadows` (`self.RotatingLight_02`) true)
          (else
            (`LightComponentBase.SetCastShadows` (`self.RotatingLight_02`) false)
            (`LightComponentBase.SetCastShadows` (`self.RotatingLight_01`) false)))
        (else
          (`SceneComponent.SetVisibility` (`self.RotatingLight_02`) false false)
          (`SceneComponent.SetVisibility` (`self.RotatingLight_01`) false false)
          (set `self.ShowcaseLightsRotate?` false))))))