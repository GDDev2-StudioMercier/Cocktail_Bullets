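; BP_ZombieAI_Master is the master Blueprint for a modular zombie AI character built from separate top, bottom and hair skeletal meshes.
; The construction script makes those parts follow the main Mesh through leader pose so they animate together.
; When the main mesh has no skeletal mesh, it has the BPC_OutfitControl component, if present, randomize the zombie before linking the parts.
; SetBonePhysics is an empty function.
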(fn `SetBonePhysics`)

(fn `UserConstructionScript`
  (bind _returnvalue (`self.GetComponentByClass` self "/Game/YI_ModularZombies/Blueprints/Master/Components/BPC_OutfitControl.BPC_OutfitControl_C"))
  (`/Engine/EditorBlueprintResources/StandardMacros.IsValid` (`SkinnedMeshComponent.SkeletalMesh` (`self.Mesh`))
    (:`Is Valid`
      _)
    (:`Is Not Valid`
      (`/Engine/EditorBlueprintResources/StandardMacros.IsValid` _returnvalue
        (:`Is Valid`
          (`/Game/YI_ModularZombies/Blueprints/Master/Components/BPC_OutfitControl.Randomize Selected Zombie` _returnvalue)))))
  (`SkinnedMeshComponent.SetLeaderPoseComponent` (`self.SK_Top`) (`self.Mesh`) true false)
  (`SkinnedMeshComponent.SetLeaderPoseComponent` (`self.SK_Bottom`) (`self.Mesh`) true false)
  (`SkinnedMeshComponent.SetLeaderPoseComponent` (`self.SK_Hair`) (`self.Mesh`) true false))