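; Showcase actor for the modular Zombie M03 character, previewing mesh and material variants under optional rotating lights.
; The construction script sets the skeletal mesh from the selected type, then applies body and head materials by slot name, matching head materials to the type.
; It also toggles the two showcase lights and their shadows, disabling rotation when they are off.
; While rotation is on, Tick yaws the Box component in increments through a Delay.
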(event `self.ReceiveTick`
  (params (DeltaSeconds :type "Float (single-precision)"))
  (bind _box (`self.Box`))
  (bind (_returnvalue_roll _returnvalue_pitch _returnvalue_yaw) (`KismetMathLibrary.BreakRotator` (`SceneComponent.K2_GetComponentRotation` _box)))
  (if (`self.ShowcaseLightsRotate?`)
    (`KismetSystemLibrary.Delay` (`self.RotationTickDelay`))
    (`SceneComponent.K2_SetWorldRotation` _box (`KismetMathLibrary.MakeRotator` _returnvalue_roll _returnvalue_pitch (+ _returnvalue_yaw (`self.RotationPerTick`))) false false)))

(fn `UserConstructionScript`
  (bind _sk_zombiemale03 (`self.SK_ZombieMale03`))
  (bind _sk_zombiemale03_2 (`self.SK_ZombieMale03`))
  (bind _sk_zombiemale03_3 (`self.SK_ZombieMale03`))
  (bind _selectzombie (`self.SelectZombie`))
  (`|ExecutionSequence`
    (:`then_0`
      ;[1 1 1] Select Mesh Options
      (switch `/Game/Migrate/YI_ModularZombies/Blueprints/ZombieM03/ZombieShowcase/Enums/E_ZombieType` (`self.SelectZombie`)
        (:`NewEnumerator0`
          (`SkinnedMeshComponent.SetSkinnedAssetAndUpdate` _sk_zombiemale03 "/Game/Migrate/YI_ModularZombies/Meshes/ZombieM03/Zombie/SK_Zombie_M03_01.SK_Zombie_M03_01" true))
        (:`NewEnumerator1`
          (`SkinnedMeshComponent.SetSkinnedAssetAndUpdate` _sk_zombiemale03 "/Game/Migrate/YI_ModularZombies/Meshes/ZombieM03/Zombie/SK_Zombie_M03_03.SK_Zombie_M03_03" true))
        (:`NewEnumerator2`
          (`SkinnedMeshComponent.SetSkinnedAssetAndUpdate` _sk_zombiemale03 "/Game/Migrate/YI_ModularZombies/Meshes/ZombieM03/Zombie/SK_Zombie_M03_02.SK_Zombie_M03_02" true))
        (:`NewEnumerator3`
          (`SkinnedMeshComponent.SetSkinnedAssetAndUpdate` _sk_zombiemale03 "/Game/Migrate/YI_ModularZombies/Meshes/ZombieM03/Zombie/SK_Zombie_M03_04.SK_Zombie_M03_04" true))))
    (:`then_1`
      (`|ExecutionSequence`
        (:`then_0`
          ;[1 1 1] Body
          (switch `/Game/Migrate/YI_ModularZombies/Blueprints/ZombieM03/ZombieShowcase/Enums/E_ZombieMaterialVariations` (`self.Select Zombie Base Material`)
            (:`NewEnumerator0`
              (`PrimitiveComponent.SetMaterialByName` _sk_zombiemale03_2 "Body" "/Game/Migrate/YI_ModularZombies/Materials/ZombieM03/Body/MI_Body_Zombie_M03_01.MI_Body_Zombie_M03_01"))
            (:`NewEnumerator6`
              (`PrimitiveComponent.SetMaterialByName` _sk_zombiemale03_2 "Body" "/Game/Migrate/YI_ModularZombies/Materials/ZombieM03/Body/MI_Body_Zombie_M03_01_NoGore.MI_Body_Zombie_M03_01_NoGore"))
            (:`NewEnumerator7`
              (`PrimitiveComponent.SetMaterialByName` _sk_zombiemale03_2 "Body" "/Game/Migrate/YI_ModularZombies/Materials/ZombieM03/Body/MI_Body_Zombie_M03_02.MI_Body_Zombie_M03_02"))
            (:`NewEnumerator8`
              (`PrimitiveComponent.SetMaterialByName` _sk_zombiemale03_2 "Body" "/Game/Migrate/YI_ModularZombies/Materials/ZombieM03/Body/MI_Body_Zombie_M03_02_NoGore.MI_Body_Zombie_M03_02_NoGore"))
            (:`NewEnumerator11`
              (`PrimitiveComponent.SetMaterialByName` _sk_zombiemale03_2 "Body" "/Game/Migrate/YI_ModularZombies/Materials/ZombieM03/Body/MI_Body_Zombie_M03_03.MI_Body_Zombie_M03_03"))
            (:`NewEnumerator12`
              (`PrimitiveComponent.SetMaterialByName` _sk_zombiemale03_2 "Body" "/Game/Migrate/YI_ModularZombies/Materials/ZombieM03/Body/MI_Body_Zombie_M03_03_NoGore.MI_Body_Zombie_M03_03_NoGore"))))
        (:`then_1`
          ;[1 1 1] HeadVariations
          (switch `/Game/Migrate/YI_ModularZombies/Blueprints/ZombieM03/ZombieShowcase/Enums/E_ZombieHeadVariations` (`self.Select Zombie Head Base Material`)
            (:`NewEnumerator0`
              (switch `/Game/Migrate/YI_ModularZombies/Blueprints/ZombieM03/ZombieShowcase/Enums/E_ZombieType` _selectzombie
                (:`NewEnumerator0`
                  (`PrimitiveComponent.SetMaterialByName` _sk_zombiemale03_3 "Head" "/Game/Migrate/YI_ModularZombies/Materials/ZombieM03/Head01/MI_Head01_Zombie_M03_01.MI_Head01_Zombie_M03_01" :!label _label))
                (:`NewEnumerator1`
                  (goto _label))
                (:`NewEnumerator2`
                  (`PrimitiveComponent.SetMaterialByName` _sk_zombiemale03_3 "Head" "/Game/Migrate/YI_ModularZombies/Materials/ZombieM03/Head02/MI_Head02_Zombie_M03_01.MI_Head02_Zombie_M03_01" :!label _label_2))
                (:`NewEnumerator3`
                  (goto _label_2))))
            (:`NewEnumerator6`
              (switch `/Game/Migrate/YI_ModularZombies/Blueprints/ZombieM03/ZombieShowcase/Enums/E_ZombieType` _selectzombie
                (:`NewEnumerator0`
                  (`PrimitiveComponent.SetMaterialByName` _sk_zombiemale03_3 "Head" "/Game/Migrate/YI_ModularZombies/Materials/ZombieM03/Head01/MI_Head01_Zombie_M03_01_NoGore.MI_Head01_Zombie_M03_01_NoGore" :!label _label_3))
                (:`NewEnumerator1`
                  (goto _label_3))
                (:`NewEnumerator2`
                  (`PrimitiveComponent.SetMaterialByName` _sk_zombiemale03_3 "Head" "/Game/Migrate/YI_ModularZombies/Materials/ZombieM03/Head02/MI_Head02_Zombie_M03_01_NoGore.MI_Head02_Zombie_M03_01_NoGore" :!label _label_4))
                (:`NewEnumerator3`
                  (goto _label_4))))
            (:`NewEnumerator7`
              (switch `/Game/Migrate/YI_ModularZombies/Blueprints/ZombieM03/ZombieShowcase/Enums/E_ZombieType` _selectzombie
                (:`NewEnumerator0`
                  (`PrimitiveComponent.SetMaterialByName` _sk_zombiemale03_3 "Head" "/Game/Migrate/YI_ModularZombies/Materials/ZombieM03/Head01/MI_Head01_Zombie_M03_02.MI_Head01_Zombie_M03_02" :!label _label_5))
                (:`NewEnumerator1`
                  (goto _label_5))
                (:`NewEnumerator2`
                  (`PrimitiveComponent.SetMaterialByName` _sk_zombiemale03_3 "Head" "/Game/Migrate/YI_ModularZombies/Materials/ZombieM03/Head02/MI_Head02_Zombie_M03_02.MI_Head02_Zombie_M03_02" :!label _label_6))
                (:`NewEnumerator3`
                  (goto _label_6))))
            (:`NewEnumerator8`
              (switch `/Game/Migrate/YI_ModularZombies/Blueprints/ZombieM03/ZombieShowcase/Enums/E_ZombieType` _selectzombie
                (:`NewEnumerator0`
                  (`PrimitiveComponent.SetMaterialByName` _sk_zombiemale03_3 "Head" "/Game/Migrate/YI_ModularZombies/Materials/ZombieM03/Head01/MI_Head01_Zombie_M03_02_NoGore.MI_Head01_Zombie_M03_02_NoGore" :!label _label_7))
                (:`NewEnumerator1`
                  (goto _label_7))
                (:`NewEnumerator2`
                  (`PrimitiveComponent.SetMaterialByName` _sk_zombiemale03_3 "Head" "/Game/Migrate/YI_ModularZombies/Materials/ZombieM03/Head02/MI_Head02_Zombie_M03_02_NoGore.MI_Head02_Zombie_M03_02_NoGore" :!label _label_8))
                (:`NewEnumerator3`
                  (goto _label_8))))
            (:`NewEnumerator11`
              (switch `/Game/Migrate/YI_ModularZombies/Blueprints/ZombieM03/ZombieShowcase/Enums/E_ZombieType` _selectzombie
                (:`NewEnumerator0`
                  (`PrimitiveComponent.SetMaterialByName` _sk_zombiemale03_3 "Head" "/Game/Migrate/YI_ModularZombies/Materials/ZombieM03/Head01/MI_Head01_Zombie_M03_03.MI_Head01_Zombie_M03_03" :!label _label_9))
                (:`NewEnumerator1`
                  (goto _label_9))
                (:`NewEnumerator2`
                  (`PrimitiveComponent.SetMaterialByName` _sk_zombiemale03_3 "Head" "/Game/Migrate/YI_ModularZombies/Materials/ZombieM03/Head02/MI_Head02_Zombie_M03_03.MI_Head02_Zombie_M03_03" :!label _label_10))
                (:`NewEnumerator3`
                  (goto _label_10))))
            (:`NewEnumerator12`
              (switch `/Game/Migrate/YI_ModularZombies/Blueprints/ZombieM03/ZombieShowcase/Enums/E_ZombieType` _selectzombie
                (:`NewEnumerator0`
                  (`PrimitiveComponent.SetMaterialByName` _sk_zombiemale03_3 "Head" "/Game/Migrate/YI_ModularZombies/Materials/ZombieM03/Head01/MI_Head01_Zombie_M03_03_NoGore.MI_Head01_Zombie_M03_03_NoGore" :!label _label_11))
                (:`NewEnumerator1`
                  (goto _label_11))
                (:`NewEnumerator2`
                  (`PrimitiveComponent.SetMaterialByName` _sk_zombiemale03_3 "Head" "/Game/Migrate/YI_ModularZombies/Materials/ZombieM03/Head02/MI_Head02_Zombie_M03_03_NoGore.MI_Head02_Zombie_M03_03_NoGore" :!label _label_12))
                (:`NewEnumerator3`
                  (goto _label_12))))))))
    (:`then_2`
      ;[1 1 1] Showcase Light Settings
      (if (`self.ShowcaseLightsOn?`)
        (`SceneComponent.SetVisibility` (`self.RotatingLight_01`) true false)
        (`SceneComponent.SetVisibility` (`self.RotatingLight_02`) true false)
        (if (`self.ShowcaseLightsShadows?`)
          (`LightComponentBase.SetCastShadows` (`self.RotatingLight_01`) true)
          (`LightComponentBase.SetCastShadows` (`self.RotatingLight_02`) true)
          (else
            (`LightComponentBase.SetCastShadows` (`self.RotatingLight_02`) false)
            (`LightComponentBase.SetCastShadows` (`self.RotatingLight_01`) false)))
        (else
          (`SceneComponent.SetVisibility` (`self.RotatingLight_02`) false false)
          (`SceneComponent.SetVisibility` (`self.RotatingLight_01`) false false)
          (set `self.ShowcaseLightsRotate?` false))))))