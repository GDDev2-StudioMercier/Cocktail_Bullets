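; BP_Gauge is a vehicle gauge component that rotates itself to show a value, such as a dashboard needle.
; UpdateGuage stores the absolute incoming value as a target, and Tick moves the current value toward it at a constant interpolation speed.
; The value's fraction of MaxValue scales a roll offset, clockwise or counterclockwise, which is combined with the rotation cached at BeginPlay.
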(event `self.ReceiveBeginPlay`
  (set `self.InitialRotation` (`self.RelativeRotation`)))

(event `self.ReceiveTick`
  (params (DeltaSeconds :type "Float (single-precision)"))
  (set `self.CurrentValue` (`KismetMathLibrary.FInterpTo_Constant` (`self.CurrentValue`) (`self.Target`) DeltaSeconds (`self.LerpSpeed`)))
  (`self.K2_SetRelativeRotation` (`KismetMathLibrary.ComposeRotators` (`self.InitialRotation`) (`KismetMathLibrary.MakeRotator` (* (/ (`self.CurrentValue`) (`self.MaxValue`)) (`self.RotationAngleToMax`) (select `bool` (`self.ClockWise`) :`false` -1.0 :`true` 1.0))))))

(event `UpdateGuage`
  (params (TargetValue :type "Float (double-precision)"))
  (set `self.Target` (`KismetMathLibrary.Abs` TargetValue)))