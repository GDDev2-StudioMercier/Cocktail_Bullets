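; Drivable police car Blueprint that adds a siren, interior computer glow, spotlight and extra lights to its parent vehicle.
; Keys H, T, K and J flip-flop these features, each through an event that calls a Multicast-named counterpart.
; The siren loops four staggered timelines driving light intensities and emissive material parameters, spins six spotlights with a Delay loop, and plays attached audio.
; BeginPlay creates a dynamic instance of the name-matched interior material for the computer glow.
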(event `SirenAnimated`
  (bind _spotlight_red02 (`self.Spotlight_Red02`))
  (bind _spotlight_red03 (`self.Spotlight_Red03`))
  (bind _spotlight_red01 (`self.Spotlight_Red01`))
  (bind _spotlight_blue02 (`self.Spotlight_Blue02`))
  (bind _spotlight_blue03 (`self.Spotlight_Blue03`))
  (bind _spotlight_blue01 (`self.Spotlight_Blue01`))
  (bind (_returnvalue_roll _returnvalue_pitch _returnvalue_yaw) (`KismetMathLibrary.BreakRotator` (`SceneComponent.K2_GetComponentRotation` _spotlight_blue03)))
  (bind (_returnvalue_roll_2 _returnvalue_pitch_2 _returnvalue_yaw_2) (`KismetMathLibrary.BreakRotator` (`SceneComponent.K2_GetComponentRotation` _spotlight_blue01)))
  (bind (_returnvalue_roll_3 _returnvalue_pitch_3 _returnvalue_yaw_3) (`KismetMathLibrary.BreakRotator` (`SceneComponent.K2_GetComponentRotation` _spotlight_blue02)))
  (bind (_returnvalue_roll_4 _returnvalue_pitch_4 _returnvalue_yaw_4) (`KismetMathLibrary.BreakRotator` (`SceneComponent.K2_GetComponentRotation` _spotlight_red01)))
  (bind (_returnvalue_roll_5 _returnvalue_pitch_5 _returnvalue_yaw_5) (`KismetMathLibrary.BreakRotator` (`SceneComponent.K2_GetComponentRotation` _spotlight_red02)))
  (bind (_returnvalue_roll_6 _returnvalue_pitch_6 _returnvalue_yaw_6) (`KismetMathLibrary.BreakRotator` (`SceneComponent.K2_GetComponentRotation` _spotlight_red03)))
  ;[0 0 0 1 36] Control Sirens
  (`TimelineComponent.SetPlayRate` (`self.SirenRed01`) (`self.SirenFlashTime`))
  (`TimelineComponent.SetPlayRate` (`self.SirenRed02`) (`self.SirenFlashTime`))
  (`TimelineComponent.SetPlayRate` (`self.SirenBlue01`) (`self.SirenFlashTime`))
  (`TimelineComponent.SetPlayRate` (`self.SirenBlue02`) (`self.SirenFlashTime`))
  (`|ExecutionSequence`
    (:`then_0`
      (if (`self.SirenEnabled`) :!label _label
        (bind (_direction _red01) (`Timeline|SirenRed01` :!via `PlayFromStart`)
          (:`Update`
            (if (`self.SirenEnabled`)
              (`LightComponent.SetIntensity` (`self.Spotlight_Red01`) (* _red01 (`self.PoliceLightIntensity`)))
              (`LightComponent.SetIntensity` (`self.Spotlight_Red03`) (* _red01 (`self.PoliceLightIntensity`)))
              (`MaterialInstanceDynamic.SetScalarParameterValue` (`self.LightMaterial`) "7.1 Emissive Strength - Red Lights 01" (* _red01 (`self.EmissionPoliceLights`)))
              (else
                (`LightComponent.SetIntensity` (`self.Spotlight_Red01`) 0.0)
                (`LightComponent.SetIntensity` (`self.Spotlight_Red03`) 0.0)
                (`MaterialInstanceDynamic.SetScalarParameterValue` (`self.LightMaterial`) "7.1 Emissive Strength - Red Lights 01" 0.0))))
          (:`Finished`
            (goto _label)))))
    (:`then_1`
      (`KismetSystemLibrary.Delay` 0.25)
      (if (`self.SirenEnabled`) :!label _label_2
        (bind (_direction_2 _red02) (`Timeline|SirenRed02` :!via `PlayFromStart`)
          (:`Update`
            (if (`self.SirenEnabled`)
              (`LightComponent.SetIntensity` (`self.SirenPointRed`) (* _red02 (`self.PoliceLightIntensity`)))
              (`LightComponent.SetIntensity` (`self.Spotlight_Red02`) (* _red02 (`self.PoliceLightIntensity`)))
              (`MaterialInstanceDynamic.SetScalarParameterValue` (`self.LightMaterial`) "7.2 Emissive Strength - Red Lights 02" (* _red02 (`self.EmissionPoliceLights`)))
              (else
                (`LightComponent.SetIntensity` (`self.SirenPointRed`) 0.0)
                (`LightComponent.SetIntensity` (`self.Spotlight_Red02`) 0.0)
                (`MaterialInstanceDynamic.SetScalarParameterValue` (`self.LightMaterial`) "7.2 Emissive Strength - Red Lights 02" 0.0))))
          (:`Finished`
            (goto _label_2)))))
    (:`then_2`
      (if (`self.SirenEnabled`) :!label _label_3
        (bind (_direction_3 _blue01) (`Timeline|SirenBlue01` :!via `PlayFromStart`)
          (:`Update`
            (if (`self.SirenEnabled`)
              (`LightComponent.SetIntensity` (`self.SirenPointBlue`) (* _blue01 (`self.PoliceLightIntensity`)))
              (`LightComponent.SetIntensity` (`self.Spotlight_Blue02`) (* _blue01 (`self.PoliceLightIntensity`)))
              (`MaterialInstanceDynamic.SetScalarParameterValue` (`self.LightMaterial`) "8.1 Emissive Strength - Blue Lights 01" (* _blue01 (`self.EmissionPoliceLights`)))
              (else
                (`LightComponent.SetIntensity` (`self.SirenPointBlue`) 0.0)
                (`LightComponent.SetIntensity` (`self.Spotlight_Blue02`) 0.0)
                (`MaterialInstanceDynamic.SetScalarParameterValue` (`self.LightMaterial`) "8.1 Emissive Strength - Blue Lights 01" 0.0))))
          (:`Finished`
            (goto _label_3)))))
    (:`then_3`
      (`KismetSystemLibrary.Delay` 0.25)
      (if (`self.SirenEnabled`) :!label _label_4
        (bind (_direction_4 _blue02) (`Timeline|SirenBlue02` :!via `PlayFromStart`)
          (:`Update`
            (if (`self.SirenEnabled`)
              (`LightComponent.SetIntensity` (`self.Spotlight_Blue03`) (* _blue02 (`self.PoliceLightIntensity`)))
              (`LightComponent.SetIntensity` (`self.Spotlight_Blue01`) (* _blue02 (`self.PoliceLightIntensity`)))
              (`MaterialInstanceDynamic.SetScalarParameterValue` (`self.LightMaterial`) "8.2 Emissive Strength - Blue Lights 02" (* _blue02 (`self.EmissionPoliceLights`)))
              (else
                (`LightComponent.SetIntensity` (`self.Spotlight_Blue03`) 0.0)
                (`LightComponent.SetIntensity` (`self.Spotlight_Blue01`) 0.0)
                (`MaterialInstanceDynamic.SetScalarParameterValue` (`self.LightMaterial`) "8.2 Emissive Strength - Blue Lights 02" 0.0))))
          (:`Finished`
            (goto _label_4)))))
    (:`then_4`
      (if (`self.SirenEnabled`) :!label _label_5
        (`|ExecutionSequence`
          (:`then_0`
            (`SceneComponent.K2_SetWorldRotation` _spotlight_blue03 (`KismetMathLibrary.MakeRotator` 0.0 0.0 (+ _returnvalue_yaw (`self.SirenRotationRate`))) false false))
          (:`then_1`
            (`SceneComponent.K2_SetWorldRotation` _spotlight_blue02 (`KismetMathLibrary.MakeRotator` 0.0 0.0 (+ _returnvalue_yaw_3 (`self.SirenRotationRate`))) false false))
          (:`then_2`
            (`SceneComponent.K2_SetWorldRotation` _spotlight_blue01 (`KismetMathLibrary.MakeRotator` 0.0 0.0 (+ _returnvalue_yaw_2 (`self.SirenRotationRate`))) false false))
          (:`then_3`
            (`SceneComponent.K2_SetWorldRotation` _spotlight_red03 (`KismetMathLibrary.MakeRotator` 0.0 0.0 (+ _returnvalue_yaw_6 (`self.SirenRotationRate`))) false false))
          (:`then_4`
            (`SceneComponent.K2_SetWorldRotation` _spotlight_red02 (`KismetMathLibrary.MakeRotator` 0.0 0.0 (+ _returnvalue_yaw_5 (`self.SirenRotationRate`))) false false))
          (:`then_5`
            (`SceneComponent.K2_SetWorldRotation` _spotlight_red01 (`KismetMathLibrary.MakeRotator` 0.0 0.0 (+ _returnvalue_yaw_4 (`self.SirenRotationRate`))) false false)))
        (`KismetSystemLibrary.Delay` 0.025)
        (goto _label_5)))))

(event `self.ReceiveTick`
  (params (DeltaSeconds :type "Float (double-precision)"))
  ;[0 0 0 1 36] Control Sirens
  (`parent.ReceiveTick` DeltaSeconds))

(event `Siren`
  (params (`Lights on?` :type Boolean))
  ;[0 0 0 1 36] Control Sirens
  (`self.Multicast Siren` `Lights on?`))

(event `Key|H`
  (params (Key :type "Key Structure"))
  ;[0 0 0 1 36] Control Sirens
  (:`Pressed`
    (bind _isa (`/Engine/EditorBlueprintResources/StandardMacros.FlipFlop`)
      (:`A`
        _)
      (:`B`
        _))
    (`self.Siren` _isa)))

(event `Multicast Siren`
  (params (`Lights on?` :type Boolean))
  (bind _sirensound (`self.SirenSound`))
  ;[0 0 0 1 36] Control Sirens
  (set `self.SirenEnabled` `Lights on?`)
  (`self.SirenAnimated`)
  (if (`self.SirenEnabled`)
    (bind _returnvalue (`GameplayStatics.SpawnSoundAttached` "/Game/YI_ModularVehicles/Sounds/Master/Driving/SFX_Siren_Cue.SFX_Siren_Cue" (`self.Mesh`) "None" (0.0 0.0 0.0) (struct) "KeepRelativeOffset" false 1.0 1.0 0.0 null null))
    (set `self.SirenSound` _returnvalue)
    (else
      (`/Engine/EditorBlueprintResources/StandardMacros.IsValid` _sirensound
        (:`Is Valid`
          (`AudioComponent.Stop` _sirensound))))))

(event `Key|T`
  (params (Key :type "Key Structure"))
  ;[0 0 0 1 36] Enable Interior Computer
  (:`Pressed`
    (bind _isa (`/Engine/EditorBlueprintResources/StandardMacros.FlipFlop`)
      (:`A`
        _)
      (:`B`
        _))
    (`self.ToggleComputer` _isa)))

(event `ToggleComputer`
  (params (`Lights on?` :type Boolean))
  ;[0 0 0 1 36] Enable Interior Computer
  (`self.Multicast Toggle Computer` `Lights on?`))

(event `Multicast Toggle Computer`
  (params (`Lights on?` :type Boolean))
  (bind _interior_material (`self.Interior Material`))
  ;[0 0 0 1 36] Enable Interior Computer
  (if `Lights on?`
    (`MaterialInstanceDynamic.SetScalarParameterValue` _interior_material "3. Emissive Intensity" 2.0)
    (else
      (`MaterialInstanceDynamic.SetScalarParameterValue` _interior_material "3. Emissive Intensity" 0.0))))

(event `self.ReceiveBeginPlay`
  ;[0 0 0 1 36] Enable Interior Computer
  (`parent.ReceiveBeginPlay`)
  (for (_array_element _array_index) (`MeshComponent.GetMaterials` (`self.Mesh`))
    (if (`KismetStringLibrary.Contains` (`KismetSystemLibrary.GetDisplayName` _array_element) "interior")
      (bind _returnvalue (`KismetMaterialLibrary.CreateDynamicMaterialInstance` _array_element))
      (bind _output_get (set `self.Interior Material` _returnvalue))
      (`PrimitiveComponent.SetMaterial` (`self.Mesh`) _array_index _output_get)
      (break))))

(event `Spotlight lights`
  (params (`Lights on?` :type Boolean))
  ;[0 0 0 1 36] Used if vehicle has additional spotlight (e.g. police car)
  (`self.Multicast Spotlight` `Lights on?`))

(event `Key|K`
  (params (Key :type "Key Structure"))
  ;[0 0 0 1 36] Used if vehicle has additional spotlight (e.g. police car)
  (:`Pressed`
    (bind _isa (`/Engine/EditorBlueprintResources/StandardMacros.FlipFlop`)
      (:`A`
        _)
      (:`B`
        _))
    (`self.Spotlight lights` _isa)))

(event `Multicast Spotlight`
  (params (`Lights on?` :type Boolean))
  ;[0 0 0 1 36] Used if vehicle has additional spotlight (e.g. police car)
  (`LightComponent.SetIntensity` (`self.Spotlight`) (select `bool` `Lights on?` :`true` (`self.LightIntensitySpotlight`)))
  (`MaterialInstanceDynamic.SetScalarParameterValue` (`self.LightMaterial`) "5. Emissive Strength - Police Spotlight" (select `bool` `Lights on?` :`true` (`self.EmissiveIntensitySpotlight`))))

(event `BonusLights`
  (params (`Lights on?` :type Boolean))
  ;[0 0 0 1 36] Used if the vehicle has custom additional lights (e.g. police car)
  (`self.Multicast Bonus Lights` `Lights on?`))

(event `Key|J`
  (params (Key :type "Key Structure"))
  ;[0 0 0 1 36] Used if the vehicle has custom additional lights (e.g. police car)
  (:`Pressed`
    (bind _isa (`/Engine/EditorBlueprintResources/StandardMacros.FlipFlop`)
      (:`A`
        _)
      (:`B`
        _))
    (`self.BonusLights` _isa)))

(event `Multicast Bonus Lights`
  (params (`Lights on?` :type Boolean))
  ;[0 0 0 1 36] Used if the vehicle has custom additional lights (e.g. police car)
  (`LightComponent.SetIntensity` (`self.BonusLights01`) (select `bool` `Lights on?` :`true` (`self.LightIntensityBonusLight`)))
  (`LightComponent.SetIntensity` (`self.BonusLights02`) (select `bool` `Lights on?` :`true` (`self.LightIntensityBonusLight`)))
  (`MaterialInstanceDynamic.SetScalarParameterValue` (`self.LightMaterial`) "6. Emissive Strength - Police Extras" (select `bool` `Lights on?` :`true` (`self.EmissiveIntensityBonusLight`))))

(fn `UserConstructionScript`
  (`parent.UserConstructionScript`))