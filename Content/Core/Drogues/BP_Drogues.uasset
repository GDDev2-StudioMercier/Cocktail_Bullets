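; BP_Drogues is a purchasable drug card in a shop, displayed through a world-space widget that scales up on BeginPlay.
; Interact deducts the player's credits if sufficient, records the drug and plays a grow animation.
; When it ends, the card spawns a Niagara burst, passes the drug to ACStat, increments its DrugType count by map index and destroys itself.
; The last card removed makes the shop spawn new ones.
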(event `self.ReceiveBeginPlay`
  (bind _aswbp_drogues (cast `/Game/Core/Drogues/WBP_Drogues` (`WidgetComponent.GetUserWidgetObject` (`self.Widget`))))
  (set `/Game/Core/Drogues/WBP_Drogues.DrogueRef` self _aswbp_drogues)
  (bind (_direction _newtrack_0) (`Timeline|Timeline`)
    (:`Update`
      (`SceneComponent.SetWorldScale3D` (`self.Widget`) (`KismetMathLibrary.VLerp` (0.0 0.0 0.0) (1.0 0.090553 0.090553) _newtrack_0)))))

(event `/Game/Core/Characters/Player/BPI_Interact.Interact`
  (params (Player :type "/Game/Core/Characters/Player/BP_Player Object Reference"))
  (bind _droguetype (`self.DrogueType`))
  (bind _shop_ref (`self.Shop Ref`))
  (bind _playerref (`self.PlayerRef`))
  ; Buying
  (bind _output_get (set `self.PlayerRef` Player))
  (if (>= (`/Game/Core/Characters/Player/BP_Player.CreditAmount` _output_get) (`self.PriceNormal`))
    (set `/Game/Core/Characters/Player/BP_Player.CreditAmount` (- (`/Game/Core/Characters/Player/BP_Player.CreditAmount` _playerref) (`self.PriceNormal`)) _playerref)
    (`KismetArrayLibrary.Array_Add` (`/Game/Core/Characters/Player/BP_Player.Drogues` (`self.PlayerRef`)) _droguetype)
    (bind (_direction _newtrack_0) (`Timeline|Timeline_0`)
      (:`Update`
        (`SceneComponent.SetWorldScale3D` (`self.Widget`) (`KismetMathLibrary.VLerp` (`SceneComponent.K2_GetComponentScale` (`self.Widget`)) (1.1 0.10553 0.10553) _newtrack_0)))
      (:`Finished`
        (bind _returnvalue (`NiagaraFunctionLibrary.SpawnSystemAtLocation` "/Game/MixedVFX/Particles/Projectiles/Hits/NS_FairyArrow_Hit.NS_FairyArrow_Hit" (`SceneComponent.K2_GetComponentLocation` (`self.Widget`)) (struct) (0.001 0.001 0.001) true true "AutoRelease"))
        (`SceneComponent.SetWorldScale3D` _returnvalue (0.5 0.5 0.5))
        (`/Game/Core/Characters/Player/AC_Stat.Add  drogues` (`/Game/Core/Characters/Player/BP_Player.AC_Stat` (`self.PlayerRef`)) _droguetype)
        (`self.NumberOfCards` _droguetype)
        (`KismetArrayLibrary.Array_RemoveItem` (`/Game/Core/Drogues/BP_DrogueShop.DroguesInShop` _shop_ref) self)
        (if (== (`KismetArrayLibrary.Array_Length` (`/Game/Core/Drogues/BP_DrogueShop.DroguesInShop` (`self.Shop Ref`))) 0)
          (`/Game/Core/Drogues/BP_DrogueShop.SpawnNewCards` _shop_ref))
        (`self.K2_DestroyActor`)))))

(fn `NumberOfCards`
  (params (Name :type "/Game/Core/Drogues/E_DroguesName Enum" :default "NewEnumerator0"))
  (bind _drugtype (`/Game/Core/Characters/Player/BP_Player.DrugType` (`self.PlayerRef`)))
  (bind (_key _value) (`BlueprintMapLibrary.Map_GetKeyValueByIndex` _drugtype (`self.Index`)))
  (switch `/Game/Core/Drogues/E_DroguesName` Name
    (:`NewEnumerator0`
      (set `self.Index` 0))
    (:`NewEnumerator1`
      (set `self.Index` 1))
    (:`NewEnumerator2`
      (set `self.Index` 2))
    (:`NewEnumerator3`
      (set `self.Index` 3))
    (:`NewEnumerator4`
      (set `self.Index` 4))
    (:`NewEnumerator6`
      (set `self.Index` 5)))
  (`BlueprintMapLibrary.Map_Add` _drugtype _key (+ _value 1)))

(fn `UserConstructionScript`)