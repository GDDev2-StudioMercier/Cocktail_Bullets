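; Shop actor that offers three drug cards (BP_Drogues) at its slot positions.
; BeginPlay fills a pool from E_DroguesName, then calls SpawnNewCrads.
; Each refresh destroys current cards and shuffles the pool before appending the previous offers, pushing them to the back to limit repeats.
; Spawned cards receive type, index and shop reference; their types leave the pool mid-loop, so picks skip alternate entries.
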(event `self.ReceiveBeginPlay`
  (bind _enumvalue (foreach `/Game/Core/Drogues/E_DroguesName` false)
    (:`LoopBody`
      (`KismetArrayLibrary.Array_Add` (`self.DroguesTypes`) _enumvalue))
    (:`then`
      (`self.SpawnNewCrads`))))

(event `SpawnNewCrads`
  (bind (_returnvalue_roll _returnvalue_pitch _returnvalue_yaw) (`KismetMathLibrary.BreakRotator` (`self.K2_GetActorRotation`)))
  ; Spawn New Cards
  (if (not (`KismetArrayLibrary.Array_IsEmpty` (`self.DroguesInShop`)))
    (for _array_element (`self.DroguesInShop`)
      (`/Engine/EditorBlueprintResources/StandardMacros.IsValid` _array_element
        (:`Is Valid`
          (`self.K2_DestroyActor` _array_element)))))
  (`KismetArrayLibrary.Array_Clear` (`self.DroguesInShop`))
  (`KismetArrayLibrary.Array_Shuffle` (`self.DroguesTypes`))
  (for _array_element_2 (`self.DroguesTypesInShop`)
    (`KismetArrayLibrary.Array_Add` (`self.DroguesTypes`) _array_element_2))
  (`KismetArrayLibrary.Array_Clear` (`self.DroguesTypesInShop`))
  (for _index (range 3)
    (switch `int` _index
      (:`0`
        (set `self.Slot` (`self.Slot1`)))
      (:`1`
        (set `self.Slot` (`self.Slot2`)))
      (:`2`
        (set `self.Slot` (`self.Slot3`))))
    (bind _output (`|GetArrayItem` (`self.DroguesTypes`) _index))
    (bind _returnvalue (`|SpawnActorFromClass` "/Game/Core/Drogues/BP_Drogues.BP_Drogues_C" (`KismetMathLibrary.MakeTransform` (`SceneComponent.K2_GetComponentLocation` (`self.Slot`)) (`KismetMathLibrary.MakeRotator` _returnvalue_roll _returnvalue_pitch (- _returnvalue_yaw 90.0))) "Undefined" "MultiplyWithRoot" null 2500 _output self _index null))
    (`KismetArrayLibrary.Array_Add` (`self.DroguesInShop`) _returnvalue)
    (`KismetArrayLibrary.Array_Add` (`self.DroguesTypesInShop`) _output)
    (`KismetArrayLibrary.Array_Remove` (`self.DroguesTypes`) _index)))

(fn `UserConstructionScript`)