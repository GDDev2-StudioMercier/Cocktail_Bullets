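; BP_RerollDrogue is an interactable that lets the player pay credits to reroll a shop's cards.
; On BeginPlay it passes itself to the WBP_Reroll widget in its Widget component.
; Interact checks the player's CreditAmount against Cost, deducts it and calls SpawnNewCards on the referenced shop.
; Each successful reroll then raises Cost by a fixed multiplier, truncated to a whole number.
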(event `self.ReceiveBeginPlay`
  (bind _aswbp_reroll (cast `/Game/Core/Items/WBP_Reroll` (`WidgetComponent.GetUserWidgetObject` (`self.Widget`))))
  (set `/Game/Core/Items/WBP_Reroll.RerollRef` self _aswbp_reroll))

(event `/Game/Core/Characters/Player/BPI_Interact.Interact`
  (params (Player :type "/Game/Core/Characters/Player/BP_Player Object Reference"))
  (bind _playerref (`self.PlayerRef`))
  (bind _output_get (set `self.PlayerRef` Player))
  (if (>= (`/Game/Core/Characters/Player/BP_Player.CreditAmount` _output_get) (`self.Cost`))
    (set `/Game/Core/Characters/Player/BP_Player.CreditAmount` (- (`/Game/Core/Characters/Player/BP_Player.CreditAmount` _playerref) (`self.Cost`)) _playerref)
    (`/Game/Core/Drogues/BP_DrogueShop.SpawnNewCards` (`self.ShopRef`))
    (set `self.Cost` (`KismetMathLibrary.FTrunc` (* (`self.Cost`) 1.2)))))

(fn `UserConstructionScript`)