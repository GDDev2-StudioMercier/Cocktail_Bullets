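; BP_ItemShop is a shop actor that displays three BP_Item actors at its slot locations, each given an item type.
; BeginPlay fills a pool from every E_ItemTypes value, then calls SpawnNewCards.
; Each refresh destroys current items, shuffles the pool, then appends the previously shown types at the back to discourage immediate repeats.
; Spawned items receive a shop reference and index, and their types move from the pool to the in-shop list.
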(event `self.ReceiveBeginPlay`
  (bind _enumvalue (foreach `/Game/Core/Items/E_ItemTypes` false)
    (:`LoopBody`
      (`KismetArrayLibrary.Array_Add` (`self.ItemsTypes`) _enumvalue))
    (:`then`
      (`self.SpawnNewCards`))))

(event `SpawnNewCards`
  ; Spawn New Cards
  (if (not (`KismetArrayLibrary.Array_IsEmpty` (`self.ItemsInShop`)))
    (for _array_element (`self.ItemsInShop`)
      (`/Engine/EditorBlueprintResources/StandardMacros.IsValid` _array_element
        (:`Is Valid`
          (`self.K2_DestroyActor` _array_element)))))
  (`KismetArrayLibrary.Array_Clear` (`self.ItemsInShop`))
  (`KismetArrayLibrary.Array_Shuffle` (`self.ItemsTypes`))
  (for _array_element_2 (`self.ItemsTypesInShop`)
    (`KismetArrayLibrary.Array_Add` (`self.ItemsTypes`) _array_element_2))
  (`KismetArrayLibrary.Array_Clear` (`self.ItemsTypesInShop`))
  (for _index (range 3)
    (switch `int` _index
      (:`0`
        (set `self.Slot` (`self.Slot1`)))
      (:`1`
        (set `self.Slot` (`self.Slot2`)))
      (:`2`
        (set `self.Slot` (`self.Slot3`))))
    (bind _output (`|GetArrayItem` (`self.ItemsTypes`) _index))
    (bind _returnvalue (`|SpawnActorFromClass` "/Game/Core/Items/BP_Item.BP_Item_C" (`KismetMathLibrary.MakeTransform` (`SceneComponent.K2_GetComponentLocation` (`self.Slot`))) "Undefined" "MultiplyWithRoot" null _output true self _index null))
    (`KismetArrayLibrary.Array_Add` (`self.ItemsInShop`) _returnvalue)
    (`KismetArrayLibrary.Array_Add` (`self.ItemsTypesInShop`) _output)
    (`KismetArrayLibrary.Array_Remove` (`self.ItemsTypes`) _index)))

(fn `UserConstructionScript`)