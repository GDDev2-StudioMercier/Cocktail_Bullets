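; BP_ItemUpgradeShop is a shop actor that displays upgrade cards for items the player holds.
; It caches the BP_Player pawn on BeginPlay.
; Each AddUpgradeCard call spawns a non-normal BP_Item for the player's item at the current Index, placed at one of four slot components and yawed relative to the shop.
; It records the spawned card and its type in arrays, then increments Index for the next call.
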(event `self.ReceiveBeginPlay`
  (bind _asbp_player (cast `/Game/Core/Characters/Player/BP_Player` (`GameplayStatics.GetPlayerPawn` 0)))
  (set `self.PlayerRef` _asbp_player))

(event `AddUpgradeCard`
  (bind (_returnvalue_roll _returnvalue_pitch _returnvalue_yaw) (`KismetMathLibrary.BreakRotator` (`self.K2_GetActorRotation`)))
  (bind _output (`|GetArrayItem` (`/Game/Core/Characters/Player/BP_Player.Items` (`self.PlayerRef`)) (`self.Index`)))
  ; Spawn New Cards
  (bind _returnvalue (`|SpawnActorFromClass` "/Game/Core/Items/BP_Item.BP_Item_C" (`KismetMathLibrary.MakeTransform` (`SceneComponent.K2_GetComponentLocation` (select `int` (`self.Index`) :`0` (`self.Slot1`) :`1` (`self.Slot2`) :`2` (`self.Slot3`) :`3` (`self.Slot4`))) (`KismetMathLibrary.MakeRotator` 0.0 0.0 (- _returnvalue_yaw 90.0))) "Undefined" "MultiplyWithRoot" null _output false null 0 null null))
  (`KismetArrayLibrary.Array_Add` (`self.ItemsInUpgradeShop`) _returnvalue)
  (`KismetArrayLibrary.Array_Add` (`self.ItemsTypesInUpgradeShop`) _output)
  (`/Engine/EditorBlueprintResources/StandardMacros.IncrementInt` (`self.Index`)))

(fn `UserConstructionScript`)