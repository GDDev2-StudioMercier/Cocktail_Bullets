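; Player stat component that applies the boosts granted by drug ("Drogues") items.
; Adddrogues looks up the drug's row in DT_Drogues by enum name, then applies its two typed modifiers in sequence, calling Player.UpdateStats after each.
; Helper functions add each value to the player's life, fire rate, walk speed, damage or reload boost.
; NumberOfCards increments only when the second modifier is Vie (life).
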(event `init`
  (params (player :type "/Game/Core/Characters/Player/BP_Player Object Reference"))
  (set `self.Player` player))

(event `Add  drogues`
  (params (DrogueName :type "/Game/Developers/miche/Drogues/E_DroguesName Enum" :default "NewEnumerator0"))
  (bind _player (`self.Player`))
  (bind _output_get (set `self.Drogue Name` DrogueName))
  (bind _returnvalue (`|GetDataTableRow` "/Game/Developers/miche/Drogues/DT_Drogues.DT_Drogues" (`KismetStringLibrary.Conv_StringToName` (`|GetEnumeratorNameAsString` _output_get)))
    (:`then`
      (switch `/Game/Developers/miche/Drogues/E_DroguesType` (`.Type1_23_AB0FE2244AA4010676C1E88E281B5F4B` (break `/Game/Developers/miche/Drogues/S_Drogues` _returnvalue))
        (:`NewEnumerator0`
          (bind _returnvalue_2 (* 1.0 (`.Data_Type1_24_550060E74245568DCF5FDC96C13E123C` (break `/Game/Developers/miche/Drogues/S_Drogues` _returnvalue))))
          (`self.Vie` _player _returnvalue_2))
        (:`NewEnumerator1`
          (`self.FireRate` _player _returnvalue_2))
        (:`NewEnumerator2`
          (`self.Speed` _player _returnvalue_2))
        (:`NewEnumerator4`
          (`self.Degats` _player _returnvalue_2))
        (:`NewEnumerator5`
          (`self.Reload` _player _returnvalue_2)))
      (`/Game/Core/Characters/Player/BP_Player.UpdateStats` _player)
      (switch `/Game/Developers/miche/Drogues/E_DroguesType` (`.Type2_18_224A64654EA14DE954842797E5144687` (break `/Game/Developers/miche/Drogues/S_Drogues` _returnvalue))
        (:`NewEnumerator0`
          (bind _returnvalue_3 (* 1.0 (`.Data_Type2_25_5125C81B4B8F6867610813B2A16F61C2` (break `/Game/Developers/miche/Drogues/S_Drogues` _returnvalue))))
          (`self.Vie` _player _returnvalue_3)
          (set `self.NumberOfCards` (+ (`self.NumberOfCards`) 1)))
        (:`NewEnumerator1`
          (`self.FireRate` _player _returnvalue_3))
        (:`NewEnumerator2`
          (`self.Speed` _player _returnvalue_3))
        (:`NewEnumerator4`
          (`self.Degats` _player _returnvalue_3))
        (:`NewEnumerator5`
          (`self.Reload` _player _returnvalue_3)))
      (`/Game/Core/Characters/Player/BP_Player.UpdateStats` _player))))

(fn `Degats`
  (params (Player :type "/Game/Core/Characters/Player/BP_Player Object Reference") (Data :type "Float (double-precision)"))
  (set `/Game/Core/Characters/Player/BP_Player.DamageBoost` (+ Data (`/Game/Core/Characters/Player/BP_Player.DamageBoost` Player)) Player))

(fn `FireRate`
  (params (Player :type "/Game/Core/Characters/Player/BP_Player Object Reference") (Data :type "Float (double-precision)"))
  (set `/Game/Core/Characters/Player/BP_Player.FireRateBoost` (+ Data (`/Game/Core/Characters/Player/BP_Player.FireRateBoost` Player)) Player))

(fn `Reload`
  (params (Player :type "/Game/Core/Characters/Player/BP_Player Object Reference") (Data :type "Float (double-precision)"))
  (set `/Game/Core/Characters/Player/BP_Player.ReloadSpeedBoost` (+ Data (`/Game/Core/Characters/Player/BP_Player.ReloadSpeedBoost` Player)) Player))

(fn `Speed`
  (params (Player :type "/Game/Core/Characters/Player/BP_Player Object Reference") (Data :type "Float (double-precision)"))
  (set `/Game/Core/Characters/Player/BP_Player.WalkSpeedBoost` (+ Data (`/Game/Core/Characters/Player/BP_Player.WalkSpeedBoost` Player)) Player))

(fn `Vie`
  (params (Player :type "/Game/Core/Characters/Player/BP_Player Object Reference") (Data :type "Float (double-precision)"))
  (set `/Game/Core/Characters/Player/BP_Player.LifeBoost` (+ Data (`/Game/Core/Characters/Player/BP_Player.LifeBoost` Player)) Player))