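; Ravageur boss character that drives a boss health bar on the player's widget and can dash.
; A timeline fills the bar on BeginPlay; taking a shot stops that fill or updates the bar from HP.
; Dash sphere-traces toward the player when attacking, otherwise in a random local direction, then lerps to the hit or end point.
; Dash play rate scales with the Speed stat and blocked distance, with a DoOnce preventing overlapping dashes.
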(event `self.ReceiveBeginPlay`
  (bind _widget (`self.Widget`))
  (bind _healthbar (`/Game/UI/widgets/WBP_GameUI1.HealthBar` _widget))
  (`parent.ReceiveBeginPlay`)
  (bind _asbp_player (cast `/Game/Core/Characters/Player/BP_Player` (`GameplayStatics.GetPlayerPawn` 0)))
  (set `self.Widget` (`/Game/Core/Characters/Player/BP_Player.Widget` _asbp_player))
  (bind (_direction _alpha) (`Timeline|HealthBar` :!via `PlayFromStart`)
    (:`Update`
      (`ProgressBar.SetPercent` _healthbar (`KismetMathLibrary.Lerp` 0.0 1.0 _alpha)))
    (:`Finished`
      (`ProgressBar.SetPercent` _healthbar (/ (`BlueprintMapLibrary.Map_Find` (`self.Stats`) "HP") (`/Game/UI/widgets/WBP_GameUI1.MaxHealth` _widget))))))

(event `Dash`
  (params (bIsAttacking :type Boolean))
  (bind _returnvalue (`self.GetActorForwardVector`))
  (bind _returnvalue_2 (`self.GetActorRightVector`))
  (bind _returnvalue_3 (`self.K2_GetActorLocation`))
  (set `self.bIsDashing` true)
  (`/Engine/EditorBlueprintResources/StandardMacros.DoOnce` false :!label _label
    (:`Completed`
      (bind _outhit (`KismetSystemLibrary.SphereTraceSingle` :`Start` _returnvalue_3 :`End` (`KismetMathLibrary.SelectVector` (`self.K2_GetActorLocation` (`GameplayStatics.GetPlayerPawn` 0)) (+ _returnvalue_3 (* (`KismetArrayLibrary.Array_Random` (`|MakeArray` _returnvalue (* _returnvalue -1.0) _returnvalue_2 (* _returnvalue_2 -1.0))) (`self.DashLenght`))) bIsAttacking) :`Radius` 5.0 :`TraceChannel` "TraceTypeQuery1" :`DrawDebugType` "ForDuration"))
      (bind (_bblockinghit _binitialoverlap _time _distance _location _impactpoint _normal _impactnormal _physmat _hitactor _hitcomponent _hitbonename _bonename _hititem _elementindex _faceindex _tracestart _traceend) (`GameplayStatics.BreakHitResult` _outhit))
      (bind _output_get (set `self.CurrentPlayrate` (* (`self.DashSpeed(s)`) (/ (`BlueprintMapLibrary.Map_Find` (`self.Stats`) "Speed") (`BlueprintMapLibrary.Map_Find` (`self.BaseStats`) "Speed")) (select `bool` _bblockinghit :`false` 1.0 :`true` (/ (`self.DashLenght`) (`KismetMathLibrary.Vector_Distance` _tracestart _impactpoint))))))
      (`TimelineComponent.SetPlayRate` (`self.Dashing`) _output_get)
      (bind (_direction _alpha) (`Timeline|Dashing` :!via `PlayFromStart`)
        (:`Update`
          (`self.K2_SetActorLocation` (`KismetMathLibrary.VLerp` _tracestart (`KismetMathLibrary.SelectVector` _impactpoint _traceend _bblockinghit) _alpha)))
        (:`Finished`
          (set `self.bIsDashing` false)
          (goto _label :!via `Reset`))))))

(event `/Game/Core/Characters/Player/BPI_Shot.Shot`
  (params (Player :type "/Game/Core/Characters/Player/BP_Player Object Reference") (Damage :type "Float (double-precision)") (CritDamage :type "Float (double-precision)") (MultiCredit :type "Float (double-precision)"))
  (bind _widget (`self.Widget`))
  (bind _healthbar (`self.HealthBar`))
  (`parent.Shot` Player Damage CritDamage MultiCredit)
  (if (`TimelineComponent.IsPlaying` _healthbar)
    (`TimelineComponent.Stop` _healthbar)
    (else
      (`ProgressBar.SetPercent` (`/Game/UI/widgets/WBP_GameUI1.HealthBar` _widget) (/ (`BlueprintMapLibrary.Map_Find` (`self.Stats`) "HP") (`/Game/UI/widgets/WBP_GameUI1.MaxHealth` _widget))))))

(fn `UserConstructionScript`
  (`parent.UserConstructionScript`))