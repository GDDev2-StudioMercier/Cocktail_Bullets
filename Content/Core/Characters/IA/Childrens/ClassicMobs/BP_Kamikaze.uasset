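; BP_Kamikaze is an AI mob whose custom attack is a suicide blast, fired after a half-second timer.
; It checks actors overlapping its Sphere, damaging BPI_Shot implementers with the player's Damage and crediting the player at a reduced multiplier.
; A player without that interface takes the mob's own Damage stat, and only that hit spawns the explosion effect.
; The mob destroys itself after the check.
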(event `CustomAttack`
  (`KismetSystemLibrary.K2_SetTimerDelegate` (delegate `CheckRadius`) 0.5))

(event `CheckRadius`
  (bind _asbp_player (cast `/Game/Core/Characters/Player/BP_Player` (`GameplayStatics.GetPlayerPawn` 0) :!pure true))
  (for _array_element (`PrimitiveComponent.GetOverlappingActors` (`self.Sphere`) null)
    (if (`KismetSystemLibrary.DoesImplementInterface` _array_element "/Game/Core/Characters/Player/BPI_Shot.BPI_Shot_C")
      (message `/Game/Core/Characters/Player/BPI_Shot.Shot` _array_element _asbp_player (`/Game/Core/Characters/Player/BP_Player.Damage` _asbp_player) 1.0 0.5)
      (elif (== _array_element _asbp_player)
        (`/Game/Core/Characters/Player/BP_Player.ReceiveDamage` _asbp_player (`BlueprintMapLibrary.Map_Find` (`self.Stats`) "Damage"))
        (`NiagaraFunctionLibrary.SpawnSystemAtLocation` "/Game/MixedVFX/Particles/Explosions/NS_ExplosionGroundBig.NS_ExplosionGroundBig" (`self.K2_GetActorLocation`)))))
  (`self.K2_DestroyActor`))

(fn `UserConstructionScript`
  (`parent.UserConstructionScript`))