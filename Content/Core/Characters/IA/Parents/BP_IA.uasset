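; Parent AI enemy character for a wave-based game that takes shots, attacks and pays the player credits on death.
; BeginPlay scales base stats by the current wave using per-stat upgrades and divisors, rounding all but attack speed.
; Shot reduces HP until GetKilled updates kills and wave-scaled money, triggers KillAllAI for bosses, then plays a death montage or ragdolls before destruction.
; An Attacking macro plays a random attack montage.
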(event `self.ReceiveBeginPlay`
  (bind _currentwave (`/Game/Core/GameParameters/GM_Game.CurrentWave` (`self.As GM Game`)))
  ; Initialisation
  (bind _asgm_game (cast `/Game/Core/GameParameters/GM_Game` (`GameplayStatics.GetGameMode`)))
  (set `self.As GM Game` _asgm_game)
  (bind (_keypin _valuepin) (`|MapForEach` (`self.BaseStats`))
    (:`then`
      (`/Engine/EditorBlueprintResources/StandardMacros.IncrementInt` (`self.Index`)
        (:`  `
          (bind _returnvalue (+ _valuepin (* (`BlueprintMapLibrary.Map_Find` (`self.UpgradeStats`) _keypin) (- _currentwave 1) (/ _currentwave (select `int` (`self.Index`) :`0` 5.0 :`1` 7.0 :`2` 6.0 :`3` 10.0 :`4` 7.0)))))
          (`BlueprintMapLibrary.Map_Add` (`self.Stats`) _keypin (`KismetMathLibrary.SelectFloat` _returnvalue (`KismetMathLibrary.Conv_IntToDouble` (`KismetMathLibrary.Round` _returnvalue)) (`KismetStringLibrary.Contains` _keypin "AttackSpeed"))))))
    (:`CompletedPin`
      (set `CharacterMovementComponent.MaxWalkSpeed` (`BlueprintMapLibrary.Map_Find` (`self.Stats`) "Speed") (`self.CharacterMovement`)))))

(event `GetKilled`
  (params (CreditMultiplier :type "Float (double-precision)"))
  (bind _moneydrop (`self.MoneyDrop`))
  (bind _deathanim (`self.DeathAnim`))
  (bind _returnvalue (`KismetMathLibrary.Conv_IntToDouble` (`/Game/Core/GameParameters/GM_Game.CurrentWave` (`self.As GM Game`))))
  ; Death
  (if (not (not (`self.bIsBoss?`)))
    (`/Game/Core/GameParameters/GM_Game.KillAllAI` (`self.As GM Game`) self))
  (bind _asbp_player (cast `/Game/Core/Characters/Player/BP_Player` (`GameplayStatics.GetPlayerPawn` 0)))
  (`/Engine/EditorBlueprintResources/StandardMacros.IncrementInt` (`/Game/UI/widgets/WBP_GameUI.KillCount` (`/Game/Core/Characters/Player/BP_Player.Widget` _asbp_player))
    (:`  `
      (bind _output_get (set `/Game/Core/Characters/Player/BP_Player.CreditAmount` (+ (`/Game/Core/Characters/Player/BP_Player.CreditAmount` _asbp_player) (`KismetMathLibrary.Round` (* (+ (`KismetMathLibrary.Conv_IntToDouble` _moneydrop) (* (/ (`KismetMathLibrary.Conv_IntToDouble` _moneydrop) 10.0) (- _returnvalue 1.0) (+ 1.0 (* 0.06 _returnvalue)))) CreditMultiplier))) _asbp_player))
      (`KismetSystemLibrary.PrintString` (`KismetStringLibrary.Conv_IntToString` _output_get) true false)
      (bind _asbp_player_2 (cast `/Game/Core/Characters/Player/BP_Player` (`GameplayStatics.GetPlayerPawn` 0)))
      (`TextBlock.SetText` (`/Game/UI/widgets/WBP_GameUI.Money` (`/Game/Core/Characters/Player/BP_Player.Widget` _asbp_player_2)) (`KismetTextLibrary.Conv_IntToText` _output_get))
      (set `CharacterMovementComponent.MaxWalkSpeed` 0.0 (`self.CharacterMovement`))
      (`PrimitiveComponent.SetCollisionEnabled` (`self.CapsuleComponent`) "NoCollision")
      (`AIController.RunBehaviorTree` (cast `AIController` (`self.GetController`) :!pure true) null)
      (`/Engine/EditorBlueprintResources/StandardMacros.IsValid` _deathanim
        (:`Is Valid`
          (`|PlayMontage` (`self.Mesh`) _deathanim
            (:`OnCompleted`
              _)))
        (:`Is Not Valid`
          (`PrimitiveComponent.SetSimulatePhysics` (`self.Mesh`) true)
          (`KismetSystemLibrary.Delay` 3.0)))
      (`self.K2_DestroyActor`))))

(event `/Game/Core/Characters/Player/BPI_Shot.Shot`
  (params (Player :type "/Game/Core/Characters/Player/BP_Player Object Reference") (Damage :type "Float (double-precision)") (CritDamage :type "Float (double-precision)") (MultiCredit :type "Float (double-precision)"))
  (bind _stats (`self.Stats`))
  (bind _returnvalue (- (`BlueprintMapLibrary.Map_Find` _stats "HP") (* Damage CritDamage)))
  (`KismetSystemLibrary.PrintString` (`KismetStringLibrary.Conv_DoubleToString` _returnvalue) true false)
  (if (> _returnvalue 0.0)
    (`BlueprintMapLibrary.Map_Add` _stats "HP" _returnvalue)
    (else
      (`self.GetKilled` MultiCredit))))

(fn `UserConstructionScript`
  (set `self.AIControllerClass` (`self.AI Controller Class`)))