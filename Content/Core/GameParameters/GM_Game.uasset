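; Game mode that runs enemy waves and the timed boss spawn.
; InitWave advances the wave, grows the enemy count and starts a looping spawn timer; each enemy type comes from a 1–100 roll against ordered thresholds in DT_EnemyChancesSpawning, capped at the Wave_5+ row.
; A one-minute timer from BeginPlay stops that spawning and places BP_Ravageur at a random boss location.
; KillAllAI destroys every BP_IA except the given boss.
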(event `self.ReceiveBeginPlay`
  (bind _outactors (`GameplayStatics.GetAllActorsOfClass` "/Game/Core/Spawners/BP_EnemySpawnLocation.BP_EnemySpawnLocation_C"))
  (set `self.EnemiesSpawnLoc` _outactors)
  (bind _outactors_2 (`GameplayStatics.GetAllActorsOfClass` "/Game/Core/Spawners/BP_BossSpawnLoc.BP_BossSpawnLoc_C"))
  (set `self.BossSpawnLoc` _outactors_2)
  (`self.InitWave`)
  (`KismetSystemLibrary.K2_SetTimerDelegate` (delegate `SpawnBoss`) 60.0))

(event `SpawnBoss`
  (`KismetSystemLibrary.K2_ClearAndInvalidateTimerHandle` (`self.EnemiesSpawningTimer`))
  (`KismetSystemLibrary.PrintString` "je fais spawn le boss" true false)
  (`|SpawnActorFromClass` (select `int` (`KismetMathLibrary.RandomIntegerInRange` 0 1) :`0` "/Game/Core/Characters/IA/Childrens/Boss/BP_Ravageur.BP_Ravageur_C" :`1` "/Game/Core/Characters/IA/Childrens/Boss/BP_Ravageur.BP_Ravageur_C" :!type "Actor Class Reference") (`KismetMathLibrary.MakeTransform` (`self.K2_GetActorLocation` (`KismetArrayLibrary.Array_Random` (`self.BossSpawnLoc`)))) "AdjustIfPossibleButAlwaysSpawn" "MultiplyWithRoot"))

(event `InitWave`
  ; Initiating waves + spawn of trash mobs
  (`/Engine/EditorBlueprintResources/StandardMacros.IncrementInt` (`self.CurrentWave`)
    (:`  `
      (set `self.AmountOfEnemies` (+ (`self.AmountOfEnemies`) 3))
      (`self.HandlingEnemiesSpawning`)
      (bind _returnvalue (`KismetSystemLibrary.K2_SetTimerDelegate` (delegate `HandlingEnemiesSpawning`) 10.0 true))
      (set `self.EnemiesSpawningTimer` _returnvalue))))

(event `HandlingEnemiesSpawning`
  ; Initiating waves + spawn of trash mobs
  (for _ (range 1 (+ (`self.AmountOfEnemies`) 1))
    (if (not (> (`self.CurrentWave`) 5))
      (bind _returnvalue (`|GetDataTableRow` "/Game/Core/Characters/IA/SpawningChances/DT_EnemyChancesSpawning.DT_EnemyChancesSpawning" (select `int` (`self.CurrentWave`) :`0` "None" :`1` "Wave_1" :`2` "Wave_2" :`3` "Wave_3" :`4` "Wave_4" :`5` "Wave_5+" :!type "Name"))
        (:`then`
          (bind _output_get (set `self.Out Row` _returnvalue))))
      (else
        (bind _returnvalue_2 (`|GetDataTableRow` "/Game/Core/Characters/IA/SpawningChances/DT_EnemyChancesSpawning.DT_EnemyChancesSpawning" "Wave_5+")
          (:`then`
            (set `self.Out Row` _returnvalue_2)))))
    (set `self.Current Number` (`KismetMathLibrary.RandomIntegerInRange` 1 100))
    (for _index (range 4)
      (bind (_c_sc _b_sc _k_sc _a_sc) (break `/Game/Core/Characters/IA/SpawningChances/E_Enemies` _output_get))
      (if (<= (`self.Current Number`) (select `int` _index :`0` _c_sc :`1` _b_sc :`2` _k_sc :`3` _a_sc))
        (bind _returnvalue_3 (`|SpawnActorFromClass` (`|GetArrayItem` (`self.Class`) _index) (`KismetMathLibrary.MakeTransform` (`self.K2_GetActorLocation` (`KismetArrayLibrary.Array_Random` (`self.EnemiesSpawnLoc`)))) "AdjustIfPossibleButAlwaysSpawn" "MultiplyWithRoot" null null))
        (`KismetSystemLibrary.PrintString` (`KismetSystemLibrary.GetDisplayName` _returnvalue_3) true false)
        (break)))))

(fn `KillAllAI`
  (params (`Boss ref` :type "/Game/Core/Characters/IA/Parents/BP_IA Object Reference"))
  (bind _outactors (`GameplayStatics.GetAllActorsOfClass` "/Game/Core/Characters/IA/Parents/BP_IA.BP_IA_C"))
  (bind _output_get (set `self.AllEnemiesRef` _outactors))
  (`KismetArrayLibrary.Array_RemoveItem` _output_get `Boss ref`)
  (for _array_element (`self.AllEnemiesRef`)
    (`self.K2_DestroyActor` _array_element))
  (`KismetArrayLibrary.Array_Clear` (`self.AllEnemiesRef`))
  (return))

(fn `UserConstructionScript`)