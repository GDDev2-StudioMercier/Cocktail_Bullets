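; BP_HealStation is an interactable station that sells healing to the player for credits.
; On Interact, it does nothing if life is already within a small tolerance of max.
; Otherwise, if the player can afford Price, it plays a purchase sound, applies HealedHP through UpdateLife and deducts the credits, or else plays a failure sound.
; Unconnected nodes that format price and HP labels remain in the graph.
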(event `self.ReceiveBeginPlay`)

(event `/Game/Core/Characters/Player/BPI_Interact.Interact`
  (params (Player :type "/Game/Core/Characters/Player/BP_Player Object Reference"))
  (if (not (`KismetMathLibrary.NearlyEqual_FloatFloat` (`/Game/Core/Characters/Player/BP_Player.Life` Player) (`/Game/Core/Characters/Player/BP_Player.MaxLife` Player) 0.1))
    (if (>= (`/Game/Core/Characters/Player/BP_Player.CreditAmount` Player) (`self.Price`))
      (`GameplayStatics.SpawnSound2D` "/Game/Sound_design/UI/buy_item.buy_item" 1.0 1.0 0.0 null)
      (`/Game/Core/Characters/Player/BP_Player.UpdateLife` Player (`self.HealedHP`))
      (set `/Game/Core/Characters/Player/BP_Player.CreditAmount` (- (`/Game/Core/Characters/Player/BP_Player.CreditAmount` Player) (`self.Price`)) Player)
      (else
        (`GameplayStatics.SpawnSound2D` "/Game/Sound_design/UI/can_t_buy.can_t_buy" 1.0 1.0 0.0 null)))))

(fn `UserConstructionScript`)